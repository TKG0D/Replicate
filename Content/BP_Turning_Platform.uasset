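; BP_Turning_Platform is a rotating platform that can be frozen briefly, with a Stasis-style sound cue.
; Its RotatingMovement component turns on at BeginPlay.
; The Start event, gated by IsTurningTrue, swaps the Cube to a pulsing material, plays the sound and halts rotation for a short delay.
; It then resumes rotation, restores a grid material and clears the flag, which this graph never sets again.
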(event Custom|Start
  (if (Variables|Default|GetIsTurningTrue)
    (Rendering|Material|SetMaterial (Variables|Default|GetCube) 0 "/Game/StarterContent/Materials/M_Tech_Hex_Tile_Pulse.M_Tech_Hex_Tile_Pulse")
    (Audio|PlaySound2D "/Game/DemoGame/BPMAP2/Sounds/BotW__Stasis_to_Temple_of_Time_-_Boulder_Strat-_AudioTrimmer_com_.BotW__Stasis_to_Temple_of_Time_-_Boulder_Strat-_AudioTrimmer_com_" 1.0 1.0 0.0 0 0)
    (Components|Activation|Deactivate (Variables|Default|GetRotatingMovement))
    (Utilities|FlowControl|Delay 2.0)
    (Components|Activation|Activate (Variables|Default|GetRotatingMovement) false)
    (Variables|Default|SetIsTurningTrue false)
    (Development|PrintString "Gear Resume")
    (Rendering|Material|SetMaterial (Variables|Default|GetCube) 0 "/Game/SuperGrid/StarterPack/Materials/Palette/Grids/M_SuperGrid_Default.M_SuperGrid_Default")))

(event EventBeginPlay
  (Components|Activation|SetActive (Variables|Default|GetRotatingMovement) true false))

(event Collision|EventActorBeginOverlap
  (params (OtherActor :type Actor%20Object%20Reference)))

(fn ConstructionScript)