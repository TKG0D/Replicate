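; Closet puzzle actor where clicking four button meshes, in any order, opens a linked gate.
; Interaction blends the view to the closet, shows a clickable cursor and disables player movement; IA_Back restores the player view and walking.
; Each click applies a neon material and latches a flag through DoOnce.
; Once all four flags are set, the Cube also turns neon and a one-shot Timeline lowers the Gate's cube.
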(event OnClicked(StaticMesh)
  (params (TouchedComponent :type Primitive%20Component%20Object%20Reference) (ButtonPressed :type Key%20Structure :default "None"))
  (Rendering|Material|SetMaterial (Variables|Default|GetStaticMesh) 0 "/Game/DemoGame/Materials/Neon5.Neon5")
  (Utilities|FlowControl|DoOnce false
    (:Completed
      (bind _output_get (Variables|Default|SetButtonP1 true))
      (if (Math|Boolean|ANDBoolean _output_get (stale OnClicked(Cube4) _output_get) (stale OnClicked(Cube3) _output_get) (stale OnClicked(StaticMesh1) _output_get))
        (Variables|Default|SetAllP true)
        (if (Variables|Default|GetAllP)
          (Utilities|FlowControl|Sequence
            (:then_0
              (Rendering|Material|SetMaterial (Variables|Default|GetCube) 0 "/Game/DemoGame/Materials/Neon5.Neon5")
              (if true
                (Utilities|FlowControl|DoOnce false
                  (:Completed
                    (bind _newtrack_0 (Timeline|Timeline Play)
                      (:Update
                        (Transformation|SetRelativeLocation (Variables|/Game/DemoGame/Gates/BP_Closet_1.BP_Closet_1_C|GetCube (Variables|Default|GetGate)) (Math|Vector|Lerp(Vector) "0, 0, 0" "0.000000,0.000000,-500.000000" _newtrack_0) false false)))))))
            (:then_1
              (Rendering|Material|SetMaterial (Variables|Default|GetCube) 1 "/Game/DemoGame/Materials/Neon5.Neon5"))))))))

(event OnClicked(Cube4)
  (params (TouchedComponent :type Primitive%20Component%20Object%20Reference) (ButtonPressed :type Key%20Structure :default "None"))
  (Rendering|Material|SetMaterial (Variables|Default|GetCube4) 0 "/Game/DemoGame/Materials/Neon5.Neon5")
  (Utilities|FlowControl|DoOnce false
    (:Completed
      (bind _output_get (Variables|Default|SetButtonP2 true))
      (if (Math|Boolean|ANDBoolean (stale OnClicked(StaticMesh) _output_get) _output_get (stale OnClicked(Cube3) _output_get) (stale OnClicked(StaticMesh1) _output_get))
        (Variables|Default|SetAllP true)
        (if (Variables|Default|GetAllP)
          (Utilities|FlowControl|Sequence
            (:then_0
              (Rendering|Material|SetMaterial (Variables|Default|GetCube) 0 "/Game/DemoGame/Materials/Neon5.Neon5")
              (if true
                (Utilities|FlowControl|DoOnce false
                  (:Completed
                    (bind _newtrack_0 (Timeline|Timeline Play)
                      (:Update
                        (Transformation|SetRelativeLocation (Variables|/Game/DemoGame/Gates/BP_Closet_1.BP_Closet_1_C|GetCube (Variables|Default|GetGate)) (Math|Vector|Lerp(Vector) "0, 0, 0" "0.000000,0.000000,-500.000000" _newtrack_0) false false)))))))
            (:then_1
              (Rendering|Material|SetMaterial (Variables|Default|GetCube) 1 "/Game/DemoGame/Materials/Neon5.Neon5"))))))))

(event OnClicked(Cube3)
  (params (TouchedComponent :type Primitive%20Component%20Object%20Reference) (ButtonPressed :type Key%20Structure :default "None"))
  (Rendering|Material|SetMaterial (Variables|Default|GetCube3) 0 "/Game/DemoGame/Materials/Neon5.Neon5")
  (Utilities|FlowControl|DoOnce false
    (:Completed
      (bind _output_get (Variables|Default|SetButtonP3 true))
      (if (Math|Boolean|ANDBoolean (stale OnClicked(StaticMesh) _output_get) (stale OnClicked(Cube4) _output_get) _output_get (stale OnClicked(StaticMesh1) _output_get))
        (Variables|Default|SetAllP true)
        (if (Variables|Default|GetAllP)
          (Utilities|FlowControl|Sequence
            (:then_0
              (Rendering|Material|SetMaterial (Variables|Default|GetCube) 0 "/Game/DemoGame/Materials/Neon5.Neon5")
              (if true
                (Utilities|FlowControl|DoOnce false
                  (:Completed
                    (bind _newtrack_0 (Timeline|Timeline Play)
                      (:Update
                        (Transformation|SetRelativeLocation (Variables|/Game/DemoGame/Gates/BP_Closet_1.BP_Closet_1_C|GetCube (Variables|Default|GetGate)) (Math|Vector|Lerp(Vector) "0, 0, 0" "0.000000,0.000000,-500.000000" _newtrack_0) false false)))))))
            (:then_1
              (Rendering|Material|SetMaterial (Variables|Default|GetCube) 1 "/Game/DemoGame/Materials/Neon5.Neon5"))))))))

(event OnClicked(StaticMesh1)
  (params (TouchedComponent :type Primitive%20Component%20Object%20Reference) (ButtonPressed :type Key%20Structure :default "None"))
  (Rendering|Material|SetMaterial (Variables|Default|GetStaticMesh1) 0 "/Game/DemoGame/Materials/Neon5.Neon5")
  (Utilities|FlowControl|DoOnce false
    (:Completed
      (bind _output_get (Variables|Default|SetButtonP4 true))
      (if (Math|Boolean|ANDBoolean (stale OnClicked(StaticMesh) _output_get) (stale OnClicked(Cube4) _output_get) (stale OnClicked(Cube3) _output_get) _output_get)
        (Variables|Default|SetAllP true)
        (if (Variables|Default|GetAllP)
          (Utilities|FlowControl|Sequence
            (:then_0
              (Rendering|Material|SetMaterial (Variables|Default|GetCube) 0 "/Game/DemoGame/Materials/Neon5.Neon5")
              (if true
                (Utilities|FlowControl|DoOnce false
                  (:Completed
                    (bind _newtrack_0 (Timeline|Timeline Play)
                      (:Update
                        (Transformation|SetRelativeLocation (Variables|/Game/DemoGame/Gates/BP_Closet_1.BP_Closet_1_C|GetCube (Variables|Default|GetGate)) (Math|Vector|Lerp(Vector) "0, 0, 0" "0.000000,0.000000,-500.000000" _newtrack_0) false false)))))))
            (:then_1
              (Rendering|Material|SetMaterial (Variables|Default|GetCube) 1 "/Game/DemoGame/Materials/Neon5.Neon5"))))))))

(event Input|EnhancedActionEvents|EnhancedInputActionIA_Back
  (params (ActionValue :type Vector%202D%20Structure) (ElapsedSeconds :type Float%20%28double-precision%29) (TriggeredSeconds :type Float%20%28double-precision%29) (InputAction :type Input%20Action%20Object%20Reference :default "/Game/ThirdPerson/Input/Actions/IA_Back.IA_Back"))
  (bind _returnvalue (Game|GetPlayerController 0))
  (:Started
    (Game|Player|SetViewTargetwithBlend _returnvalue (Variables|Default|GetPlayerreff) 0.5 "VTBlend_Linear" 0.0 false)
    (Variables|/Script/Engine.PlayerController|SetbEnableClickEvents _returnvalue false)
    (Variables|/Script/Engine.PlayerController|SetbShowMouseCursor _returnvalue false)
    (Pawn|Components|CharacterMovement|SetMovementMode (Variables|/Script/Engine.Character|GetCharacterMovement (Variables|Default|GetPlayerreff)) "MOVE_Walking" 0)))

(event EventBeginPlay
  (|CallParentFunction)
  (Input|EnableInput (Game|GetPlayerController 0)))

(event EventInteraction
  (bind _returnvalue (Game|GetPlayerController 0))
  (Game|Player|SetViewTargetwithBlend _returnvalue self 0.5 "VTBlend_Linear" 0.0 false)
  (Variables|/Script/Engine.PlayerController|SetbEnableClickEvents _returnvalue true)
  (Variables|/Script/Engine.PlayerController|SetbShowMouseCursor _returnvalue true)
  (Pawn|Components|CharacterMovement|DisableMovement (Variables|/Script/Engine.Character|GetCharacterMovement (Variables|Default|GetPlayerreff))))

(event EventTick
  (params (DeltaSeconds :type Float%20%28single-precision%29)))

(event Collision|EventActorBeginOverlap
  (params (OtherActor :type Actor%20Object%20Reference)))

(fn ConstructionScript)