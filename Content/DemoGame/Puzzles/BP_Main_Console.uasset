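; Main puzzle console that, on its first Interaction event, moves four referenced objects and relights a large set of floor pieces.
; A DoOnce gates a Sequence that starts four Timelines, each lerping a target's relative location from zero to 500 units up in Z.
; The same Sequence swaps the Cube material on every referenced floor actor to Neon3, each through its own hard-wired variable.
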(event EventBeginPlay)

(event EventInteraction
  (Utilities|FlowControl|DoOnce false
    (:Completed
      (Utilities|FlowControl|Sequence
        (:then_0
          (bind _newtrack_0 (Timeline|Timeline Play)
            (:Update
              (Transformation|SetRelativeLocation (Variables|/Script/Engine.Actor|GetRootComponent (Variables|Default|GetNewVar24)) (Math|Vector|Lerp(Vector) "0, 0, 0" "0.000000,0.000000,500.000000" _newtrack_0) false false))))
        (:then_1
          (bind _newtrack_0_2 (Timeline|Timeline_0 Play)
            (:Update
              (Transformation|SetRelativeLocation (Variables|/Game/DemoGame/Gates/BP_Seventh_Gate.BP_Seventh_Gate_C|GetCube (Variables|Default|GetNewVar_25)) (Math|Vector|Lerp(Vector) "0, 0, 0" "0.000000,0.000000,500.000000" _newtrack_0_2) false false))))
        (:then_2
          (bind _newtrack_0_3 (Timeline|Timeline_1 Play)
            (:Update
              (Transformation|SetRelativeLocation (Variables|/Game/DemoGame/Gates/BP_Sixth_Gate.BP_Sixth_Gate_C|GetCube (Variables|Default|GetNewVar_26)) (Math|Vector|Lerp(Vector) "0, 0, 0" "0.000000,0.000000,500.000000" _newtrack_0_3) false false))))
        (:then_3
          (bind _newtrack_0_4 (Timeline|Timeline_2 Play)
            (:Update
              (Transformation|SetRelativeLocation (Variables|/Game/DemoGame/Gates/BP_Top_Gate.BP_Top_Gate_C|GetCube (Variables|Default|GetNewVar_27)) (Math|Vector|Lerp(Vector) "0, 0, 0" "0.000000,0.000000,500.000000" _newtrack_0_4) false false))))
        (:then_4
          (Rendering|Material|SetMaterial (Variables|/Game/DemoGame/Floor/Floor.Floor_C|GetCube (Variables|Default|GetFloor1)) 0 "/Game/DemoGame/Materials/Neon3.Neon3"))
        (:then_5
          (Rendering|Material|SetMaterial (Variables|/Game/DemoGame/Floor/Floor.Floor_C|GetCube (Variables|Default|GetFloor2)) 0 "/Game/DemoGame/Materials/Neon3.Neon3"))
        (:then_6
          (Rendering|Material|SetMaterial (Variables|/Game/DemoGame/Floor/Floor.Floor_C|GetCube (Variables|Default|GetFloor3)) 0 "/Game/DemoGame/Materials/Neon3.Neon3"))
        (:then_7
          (Rendering|Material|SetMaterial (Variables|/Game/DemoGame/Floor/Floor.Floor_C|GetCube (Variables|Default|GetFloor4)) 0 "/Game/DemoGame/Materials/Neon3.Neon3"))
        (:then_8
          (Rendering|Material|SetMaterial (Variables|/Game/DemoGame/Floor/Floor.Floor_C|GetCube (Variables|Default|GetFloor4_0)) 0 "/Game/DemoGame/Materials/Neon3.Neon3"))
        (:then_9
          (Rendering|Material|SetMaterial (Variables|/Game/DemoGame/Floor/Floor.Floor_C|GetCube (Variables|Default|GetFloor4_1)) 0 "/Game/DemoGame/Materials/Neon3.Neon3"))
        (:then_10
          (Rendering|Material|SetMaterial (Variables|/Game/DemoGame/Floor/Floor.Floor_C|GetCube (Variables|Default|GetFloor4_2)) 0 "/Game/DemoGame/Materials/Neon3.Neon3"))
        (:then_11
          (Rendering|Material|SetMaterial (Variables|/Game/DemoGame/Floor/Floor.Floor_C|GetCube (Variables|Default|GetFloor4_3)) 0 "/Game/DemoGame/Materials/Neon3.Neon3"))
        (:then_12
          (Rendering|Material|SetMaterial (Variables|/Game/DemoGame/Floor/Floor.Floor_C|GetCube (Variables|Default|GetFloor4_4)) 0 "/Game/DemoGame/Materials/Neon3.Neon3"))
        (:then_13
          (Rendering|Material|SetMaterial (Variables|/Game/DemoGame/Floor/Floor.Floor_C|GetCube (Variables|Default|GetFloor4_5)) 0 "/Game/DemoGame/Materials/Neon3.Neon3"))
        (:then_14
          (Rendering|Material|SetMaterial (Variables|/Game/DemoGame/Floor/Floor.Floor_C|GetCube (Variables|Default|GetFloor4_6)) 0 "/Game/DemoGame/Materials/Neon3.Neon3"))
        (:then_15
          (Rendering|Material|SetMaterial (Variables|/Game/DemoGame/Floor/Floor.Floor_C|GetCube (Variables|Default|GetFloor4_7)) 0 "/Game/DemoGame/Materials/Neon3.Neon3"))
        (:then_16
          (Rendering|Material|SetMaterial (Variables|/Game/DemoGame/Floor/Floor.Floor_C|GetCube (Variables|Default|GetFloor4_8)) 0 "/Game/DemoGame/Materials/Neon3.Neon3"))
        (:then_17
          (Rendering|Material|SetMaterial (Variables|/Game/DemoGame/Floor/Floor.Floor_C|GetCube (Variables|Default|GetFloor4_9)) 0 "/Game/DemoGame/Materials/Neon3.Neon3"))
        (:then_18
          (Rendering|Material|SetMaterial (Variables|/Game/DemoGame/Floor/Floor.Floor_C|GetCube (Variables|Default|GetFloor4_10)) 0 "/Game/DemoGame/Materials/Neon3.Neon3"))
        (:then_19
          (Rendering|Material|SetMaterial (Variables|/Game/DemoGame/Floor/Floor.Floor_C|GetCube (Variables|Default|GetFloor4_11)) 0 "/Game/DemoGame/Materials/Neon3.Neon3"))
        (:then_20
          (Rendering|Material|SetMaterial (Variables|/Game/DemoGame/Floor/Floor.Floor_C|GetCube (Variables|Default|GetFloor4_12)) 0 "/Game/DemoGame/Materials/Neon3.Neon3"))
        (:then_21
          (Rendering|Material|SetMaterial (Variables|/Game/DemoGame/Floor/Floor.Floor_C|GetCube (Variables|Default|GetFloor4_13)) 0 "/Game/DemoGame/Materials/Neon3.Neon3"))
        (:then_22
          (Rendering|Material|SetMaterial (Variables|/Game/DemoGame/Floor/Floor.Floor_C|GetCube (Variables|Default|GetFloor4_14)) 0 "/Game/DemoGame/Materials/Neon3.Neon3"))
        (:then_23
          (Rendering|Material|SetMaterial (Variables|/Game/DemoGame/Floor/Floor.Floor_C|GetCube (Variables|Default|GetFloor4_15)) 0 "/Game/DemoGame/Materials/Neon3.Neon3"))
        (:then_24
          (Rendering|Material|SetMaterial (Variables|/Game/DemoGame/Floor/Floor.Floor_C|GetCube (Variables|Default|GetFloor4_16)) 0 "/Game/DemoGame/Materials/Neon3.Neon3"))
        (:then_25
          (Rendering|Material|SetMaterial (Variables|/Game/DemoGame/Floor/Floor.Floor_C|GetCube (Variables|Default|GetFloor4_17)) 0 "/Game/DemoGame/Materials/Neon3.Neon3"))
        (:then_26
          (Rendering|Material|SetMaterial (Variables|/Game/DemoGame/Floor/Floor.Floor_C|GetCube (Variables|Default|GetFloor4_18)) 0 "/Game/DemoGame/Materials/Neon3.Neon3"))
        (:then_27
          (Rendering|Material|SetMaterial (Variables|/Game/DemoGame/Floor/Floor.Floor_C|GetCube (Variables|Default|GetFloor4_19)) 0 "/Game/DemoGame/Materials/Neon3.Neon3"))
        (:then_28
          (Rendering|Material|SetMaterial (Variables|/Game/DemoGame/Floor/Floor.Floor_C|GetCube (Variables|Default|GetFloor4_20)) 0 "/Game/DemoGame/Materials/Neon3.Neon3"))
        (:then_29
          (Rendering|Material|SetMaterial (Variables|/Game/DemoGame/Floor/Floor.Floor_C|GetCube (Variables|Default|GetFloor4_21)) 0 "/Game/DemoGame/Materials/Neon3.Neon3"))))))

(event EventTick
  (params (DeltaSeconds :type Float%20%28single-precision%29)))

(event Collision|EventActorBeginOverlap
  (params (OtherActor :type Actor%20Object%20Reference)))

(fn ConstructionScript)