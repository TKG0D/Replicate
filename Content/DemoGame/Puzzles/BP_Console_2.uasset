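; Puzzle console where the player toggles twelve clickable cubes into a fixed pattern to open a linked door.
; Interaction blends the view to the console, shows the cursor and disables movement and shooting until IA_Back restores them.
; Each cube's FlipFlop swaps its neon material and sets a flag, with some cubes needing the alternate material.
; When all flags match, materials change, a Timeline raises the door and a gate-open widget shows briefly.
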(event OnClicked(Cube6)
  (params (TouchedComponent :type Primitive%20Component%20Object%20Reference) (ButtonPressed :type Key%20Structure :default "None"))
  (Utilities|FlowControl|FlipFlop
    (:A
      (Rendering|Material|SetMaterial (Variables|Default|GetCube6) 0 "/Game/DemoGame/Materials/Neon2.Neon2")
      (Variables|Default|SetTrue1_2 true))
    (:B
      (Rendering|Material|SetMaterial (Variables|Default|GetCube6) 0 "/Game/DemoGame/Materials/Neon.Neon")
      (Variables|Default|SetTrue1_2 false)))
  (if (Variables|Default|GetTrue1_2)
    (Variables|Default|SetIs%20open4 true)
    (if (Variables|Default|GetIs%20open4)
      (if (Math|Boolean|ANDBoolean (Variables|Default|GetIs%20open) (Variables|Default|GetIs%20open2) (Variables|Default|GetIs%20open3) (Variables|Default|GetIs%20open4) (Variables|Default|GetIs%20open5) (Variables|Default|GetIs%20open6) (Variables|Default|GetIs%20open7) (Variables|Default|GetIs%20open8) (Variables|Default|GetIs%20open9) (Variables|Default|GetIs%20open10) (Variables|Default|GetIs%20open11) (Variables|Default|GetIs%20open12)) :!label _label
        (Utilities|FlowControl|DoOnce false
          (:Completed
            (Utilities|FlowControl|Sequence
              (:then_0
                (Rendering|Material|SetMaterial (Variables|Default|GetCube) 1 "/Game/DemoGame/Materials/Neon3.Neon3"))
              (:then_1
                (Rendering|Material|SetMaterial (Variables|Default|GetCube1) 1 "/Game/DemoGame/Materials/Neon3.Neon3"))
              (:then_2
                (Rendering|Material|SetMaterial (Variables|Default|GetCube2) 1 "/Game/DemoGame/Materials/Neon3.Neon3"))
              (:then_3
                (bind _newtrack_0 (Timeline|Timeline Play)
                  (:Update
                    (Transformation|SetRelativeLocation (Variables|/Game/DemoGame/Gates/BP_Third_Gate.BP_Third_Gate_C|GetCube (Variables|Default|GetOpendoor)) (Math|Vector|Lerp(Vector) "0, 0, 0" "0.000000,0.000000,400.000000" _newtrack_0) false false)
                    (Utilities|FlowControl|DoOnce false
                      (:Completed
                        (bind _returnvalue (UserInterface|CreateWidget "/Game/DemoGame/Widgets/WB_Gate_Open.WB_Gate_Open_C"))
                        (UserInterface|Viewport|AddtoViewport _returnvalue 0)
                        (Utilities|FlowControl|Delay 5.0)
                        (Widget|RemovefromParent _returnvalue))))))
              (:then_4
                (Rendering|Material|SetMaterial (Variables|Default|GetCube14) 0 "/Game/DemoGame/Materials/Neon3.Neon3"))
              (:then_5
                (Rendering|Material|SetMaterial (Variables|Default|GetCube13) 0 "/Game/DemoGame/Materials/Neon3.Neon3"))
              (:then_6
                (Rendering|Material|SetMaterial (Variables|Default|GetCube12) 0 "/Game/DemoGame/Materials/Neon3.Neon3"))
              (:then_7
                (Rendering|Material|SetMaterial (Variables|Default|GetCube11) 0 "/Game/DemoGame/Materials/Neon3.Neon3"))
              (:then_8
                (Rendering|Material|SetMaterial (Variables|Default|GetCube6) 0 "/Game/DemoGame/Materials/Neon3.Neon3"))
              (:then_9
                (Rendering|Material|SetMaterial (Variables|Default|GetCube5) 0 "/Game/DemoGame/Materials/Neon3.Neon3"))
              (:then_10
                (Rendering|Material|SetMaterial (Variables|Default|GetCube4) 0 "/Game/DemoGame/Materials/Neon3.Neon3"))
              (:then_11
                (Rendering|Material|SetMaterial (Variables|Default|GetCube3) 0 "/Game/DemoGame/Materials/Neon3.Neon3"))
              (:then_12
                (Rendering|Material|SetMaterial (Variables|Default|GetCube8) 10 "/Game/DemoGame/Materials/Neon3.Neon3"))
              (:then_13
                (Rendering|Material|SetMaterial (Variables|Default|GetCube7) 0 "/Game/DemoGame/Materials/Neon3.Neon3"))
              (:then_14
                (Rendering|Material|SetMaterial (Variables|Default|GetCube9) 0 "/Game/DemoGame/Materials/Neon3.Neon3"))
              (:then_15
                (Rendering|Material|SetMaterial (Variables|Default|GetCube10) 0 "/Game/DemoGame/Materials/Neon3.Neon3"))
              (:then_16
                (Rendering|Material|SetMaterial (Variables|Default|GetCube8) 0 "/Game/DemoGame/Materials/Neon3.Neon3")))))))
    (else
      (Variables|Default|SetIs%20open4 false)
      (if (Variables|Default|GetIs%20open4)
        (goto _label)))))

(event OnClicked(Cube5)
  (params (TouchedComponent :type Primitive%20Component%20Object%20Reference) (ButtonPressed :type Key%20Structure :default "None"))
  (Utilities|FlowControl|FlipFlop
    (:A
      (Rendering|Material|SetMaterial (Variables|Default|GetCube5) 0 "/Game/DemoGame/Materials/Neon2.Neon2")
      (Variables|Default|SetTrue1_1 false))
    (:B
      (Rendering|Material|SetMaterial (Variables|Default|GetCube5) 0 "/Game/DemoGame/Materials/Neon.Neon")
      (Variables|Default|SetTrue1_1 true)))
  (if (Variables|Default|GetTrue1_1)
    (Variables|Default|SetIs%20open3 true)
    (if (Variables|Default|GetIs%20open3)
      (if (Math|Boolean|ANDBoolean (Variables|Default|GetIs%20open) (Variables|Default|GetIs%20open2) (Variables|Default|GetIs%20open3) (Variables|Default|GetIs%20open4) (Variables|Default|GetIs%20open5) (Variables|Default|GetIs%20open6) (Variables|Default|GetIs%20open7) (Variables|Default|GetIs%20open8) (Variables|Default|GetIs%20open9) (Variables|Default|GetIs%20open10) (Variables|Default|GetIs%20open11) (Variables|Default|GetIs%20open12)) :!label _label
        (Utilities|FlowControl|DoOnce false
          (:Completed
            (Utilities|FlowControl|Sequence
              (:then_0
                (Rendering|Material|SetMaterial (Variables|Default|GetCube) 1 "/Game/DemoGame/Materials/Neon3.Neon3"))
              (:then_1
                (Rendering|Material|SetMaterial (Variables|Default|GetCube1) 1 "/Game/DemoGame/Materials/Neon3.Neon3"))
              (:then_2
                (Rendering|Material|SetMaterial (Variables|Default|GetCube2) 1 "/Game/DemoGame/Materials/Neon3.Neon3"))
              (:then_3
                (bind _newtrack_0 (Timeline|Timeline Play)
                  (:Update
                    (Transformation|SetRelativeLocation (Variables|/Game/DemoGame/Gates/BP_Third_Gate.BP_Third_Gate_C|GetCube (Variables|Default|GetOpendoor)) (Math|Vector|Lerp(Vector) "0, 0, 0" "0.000000,0.000000,400.000000" _newtrack_0) false false)
                    (Utilities|FlowControl|DoOnce false
                      (:Completed
                        (bind _returnvalue (UserInterface|CreateWidget "/Game/DemoGame/Widgets/WB_Gate_Open.WB_Gate_Open_C"))
                        (UserInterface|Viewport|AddtoViewport _returnvalue 0)
                        (Utilities|FlowControl|Delay 5.0)
                        (Widget|RemovefromParent _returnvalue))))))
              (:then_4
                (Rendering|Material|SetMaterial (Variables|Default|GetCube14) 0 "/Game/DemoGame/Materials/Neon3.Neon3"))
              (:then_5
                (Rendering|Material|SetMaterial (Variables|Default|GetCube13) 0 "/Game/DemoGame/Materials/Neon3.Neon3"))
              (:then_6
                (Rendering|Material|SetMaterial (Variables|Default|GetCube12) 0 "/Game/DemoGame/Materials/Neon3.Neon3"))
              (:then_7
                (Rendering|Material|SetMaterial (Variables|Default|GetCube11) 0 "/Game/DemoGame/Materials/Neon3.Neon3"))
              (:then_8
                (Rendering|Material|SetMaterial (Variables|Default|GetCube6) 0 "/Game/DemoGame/Materials/Neon3.Neon3"))
              (:then_9
                (Rendering|Material|SetMaterial (Variables|Default|GetCube5) 0 "/Game/DemoGame/Materials/Neon3.Neon3"))
              (:then_10
                (Rendering|Material|SetMaterial (Variables|Default|GetCube4) 0 "/Game/DemoGame/Materials/Neon3.Neon3"))
              (:then_11
                (Rendering|Material|SetMaterial (Variables|Default|GetCube3) 0 "/Game/DemoGame/Materials/Neon3.Neon3"))
              (:then_12
                (Rendering|Material|SetMaterial (Variables|Default|GetCube8) 10 "/Game/DemoGame/Materials/Neon3.Neon3"))
              (:then_13
                (Rendering|Material|SetMaterial (Variables|Default|GetCube7) 0 "/Game/DemoGame/Materials/Neon3.Neon3"))
              (:then_14
                (Rendering|Material|SetMaterial (Variables|Default|GetCube9) 0 "/Game/DemoGame/Materials/Neon3.Neon3"))
              (:then_15
                (Rendering|Material|SetMaterial (Variables|Default|GetCube10) 0 "/Game/DemoGame/Materials/Neon3.Neon3"))
              (:then_16
                (Rendering|Material|SetMaterial (Variables|Default|GetCube8) 0 "/Game/DemoGame/Materials/Neon3.Neon3")))))))
    (else
      (Variables|Default|SetIs%20open3 false)
      (if (Variables|Default|GetIs%20open3)
        (goto _label)))))

(event OnClicked(Cube12)
  (params (TouchedComponent :type Primitive%20Component%20Object%20Reference) (ButtonPressed :type Key%20Structure :default "None"))
  (Utilities|FlowControl|FlipFlop
    (:A
      (Rendering|Material|SetMaterial (Variables|Default|GetCube12) 0 "/Game/DemoGame/Materials/Neon2.Neon2")
      (Variables|Default|SetTrue1_8 false))
    (:B
      (Rendering|Material|SetMaterial (Variables|Default|GetCube12) 0 "/Game/DemoGame/Materials/Neon.Neon")
      (Variables|Default|SetTrue1_8 true)))
  (if (Variables|Default|GetTrue1_8)
    (Variables|Default|SetIs%20open10 true)
    (if (Variables|Default|GetIs%20open10)
      (if (Math|Boolean|ANDBoolean (Variables|Default|GetIs%20open) (Variables|Default|GetIs%20open2) (Variables|Default|GetIs%20open3) (Variables|Default|GetIs%20open4) (Variables|Default|GetIs%20open5) (Variables|Default|GetIs%20open6) (Variables|Default|GetIs%20open7) (Variables|Default|GetIs%20open8) (Variables|Default|GetIs%20open9) (Variables|Default|GetIs%20open10) (Variables|Default|GetIs%20open11) (Variables|Default|GetIs%20open12)) :!label _label
        (Utilities|FlowControl|DoOnce false
          (:Completed
            (Utilities|FlowControl|Sequence
              (:then_0
                (Rendering|Material|SetMaterial (Variables|Default|GetCube) 1 "/Game/DemoGame/Materials/Neon3.Neon3"))
              (:then_1
                (Rendering|Material|SetMaterial (Variables|Default|GetCube1) 1 "/Game/DemoGame/Materials/Neon3.Neon3"))
              (:then_2
                (Rendering|Material|SetMaterial (Variables|Default|GetCube2) 1 "/Game/DemoGame/Materials/Neon3.Neon3"))
              (:then_3
                (bind _newtrack_0 (Timeline|Timeline Play)
                  (:Update
                    (Transformation|SetRelativeLocation (Variables|/Game/DemoGame/Gates/BP_Third_Gate.BP_Third_Gate_C|GetCube (Variables|Default|GetOpendoor)) (Math|Vector|Lerp(Vector) "0, 0, 0" "0.000000,0.000000,400.000000" _newtrack_0) false false)
                    (Utilities|FlowControl|DoOnce false
                      (:Completed
                        (bind _returnvalue (UserInterface|CreateWidget "/Game/DemoGame/Widgets/WB_Gate_Open.WB_Gate_Open_C"))
                        (UserInterface|Viewport|AddtoViewport _returnvalue 0)
                        (Utilities|FlowControl|Delay 5.0)
                        (Widget|RemovefromParent _returnvalue))))))
              (:then_4
                (Rendering|Material|SetMaterial (Variables|Default|GetCube14) 0 "/Game/DemoGame/Materials/Neon3.Neon3"))
              (:then_5
                (Rendering|Material|SetMaterial (Variables|Default|GetCube13) 0 "/Game/DemoGame/Materials/Neon3.Neon3"))
              (:then_6
                (Rendering|Material|SetMaterial (Variables|Default|GetCube12) 0 "/Game/DemoGame/Materials/Neon3.Neon3"))
              (:then_7
                (Rendering|Material|SetMaterial (Variables|Default|GetCube11) 0 "/Game/DemoGame/Materials/Neon3.Neon3"))
              (:then_8
                (Rendering|Material|SetMaterial (Variables|Default|GetCube6) 0 "/Game/DemoGame/Materials/Neon3.Neon3"))
              (:then_9
                (Rendering|Material|SetMaterial (Variables|Default|GetCube5) 0 "/Game/DemoGame/Materials/Neon3.Neon3"))
              (:then_10
                (Rendering|Material|SetMaterial (Variables|Default|GetCube4) 0 "/Game/DemoGame/Materials/Neon3.Neon3"))
              (:then_11
                (Rendering|Material|SetMaterial (Variables|Default|GetCube3) 0 "/Game/DemoGame/Materials/Neon3.Neon3"))
              (:then_12
                (Rendering|Material|SetMaterial (Variables|Default|GetCube8) 10 "/Game/DemoGame/Materials/Neon3.Neon3"))
              (:then_13
                (Rendering|Material|SetMaterial (Variables|Default|GetCube7) 0 "/Game/DemoGame/Materials/Neon3.Neon3"))
              (:then_14
                (Rendering|Material|SetMaterial (Variables|Default|GetCube9) 0 "/Game/DemoGame/Materials/Neon3.Neon3"))
              (:then_15
                (Rendering|Material|SetMaterial (Variables|Default|GetCube10) 0 "/Game/DemoGame/Materials/Neon3.Neon3"))
              (:then_16
                (Rendering|Material|SetMaterial (Variables|Default|GetCube8) 0 "/Game/DemoGame/Materials/Neon3.Neon3")))))))
    (else
      (Variables|Default|SetIs%20open10 false)
      (if (Variables|Default|GetIs%20open10)
        (goto _label)))))

(event OnClicked(Cube11)
  (params (TouchedComponent :type Primitive%20Component%20Object%20Reference) (ButtonPressed :type Key%20Structure :default "None"))
  (Utilities|FlowControl|FlipFlop
    (:A
      (Rendering|Material|SetMaterial (Variables|Default|GetCube11) 0 "/Game/DemoGame/Materials/Neon2.Neon2")
      (Variables|Default|SetTrue1_7 true))
    (:B
      (Rendering|Material|SetMaterial (Variables|Default|GetCube11) 0 "/Game/DemoGame/Materials/Neon.Neon")
      (Variables|Default|SetTrue1_7 false)))
  (if (Variables|Default|GetTrue1_7)
    (Variables|Default|SetIs%20open9 true)
    (if (Variables|Default|GetIs%20open9)
      (if (Math|Boolean|ANDBoolean (Variables|Default|GetIs%20open) (Variables|Default|GetIs%20open2) (Variables|Default|GetIs%20open3) (Variables|Default|GetIs%20open4) (Variables|Default|GetIs%20open5) (Variables|Default|GetIs%20open6) (Variables|Default|GetIs%20open7) (Variables|Default|GetIs%20open8) (Variables|Default|GetIs%20open9) (Variables|Default|GetIs%20open10) (Variables|Default|GetIs%20open11) (Variables|Default|GetIs%20open12)) :!label _label
        (Utilities|FlowControl|DoOnce false
          (:Completed
            (Utilities|FlowControl|Sequence
              (:then_0
                (Rendering|Material|SetMaterial (Variables|Default|GetCube) 1 "/Game/DemoGame/Materials/Neon3.Neon3"))
              (:then_1
                (Rendering|Material|SetMaterial (Variables|Default|GetCube1) 1 "/Game/DemoGame/Materials/Neon3.Neon3"))
              (:then_2
                (Rendering|Material|SetMaterial (Variables|Default|GetCube2) 1 "/Game/DemoGame/Materials/Neon3.Neon3"))
              (:then_3
                (bind _newtrack_0 (Timeline|Timeline Play)
                  (:Update
                    (Transformation|SetRelativeLocation (Variables|/Game/DemoGame/Gates/BP_Third_Gate.BP_Third_Gate_C|GetCube (Variables|Default|GetOpendoor)) (Math|Vector|Lerp(Vector) "0, 0, 0" "0.000000,0.000000,400.000000" _newtrack_0) false false)
                    (Utilities|FlowControl|DoOnce false
                      (:Completed
                        (bind _returnvalue (UserInterface|CreateWidget "/Game/DemoGame/Widgets/WB_Gate_Open.WB_Gate_Open_C"))
                        (UserInterface|Viewport|AddtoViewport _returnvalue 0)
                        (Utilities|FlowControl|Delay 5.0)
                        (Widget|RemovefromParent _returnvalue))))))
              (:then_4
                (Rendering|Material|SetMaterial (Variables|Default|GetCube14) 0 "/Game/DemoGame/Materials/Neon3.Neon3"))
              (:then_5
                (Rendering|Material|SetMaterial (Variables|Default|GetCube13) 0 "/Game/DemoGame/Materials/Neon3.Neon3"))
              (:then_6
                (Rendering|Material|SetMaterial (Variables|Default|GetCube12) 0 "/Game/DemoGame/Materials/Neon3.Neon3"))
              (:then_7
                (Rendering|Material|SetMaterial (Variables|Default|GetCube11) 0 "/Game/DemoGame/Materials/Neon3.Neon3"))
              (:then_8
                (Rendering|Material|SetMaterial (Variables|Default|GetCube6) 0 "/Game/DemoGame/Materials/Neon3.Neon3"))
              (:then_9
                (Rendering|Material|SetMaterial (Variables|Default|GetCube5) 0 "/Game/DemoGame/Materials/Neon3.Neon3"))
              (:then_10
                (Rendering|Material|SetMaterial (Variables|Default|GetCube4) 0 "/Game/DemoGame/Materials/Neon3.Neon3"))
              (:then_11
                (Rendering|Material|SetMaterial (Variables|Default|GetCube3) 0 "/Game/DemoGame/Materials/Neon3.Neon3"))
              (:then_12
                (Rendering|Material|SetMaterial (Variables|Default|GetCube8) 10 "/Game/DemoGame/Materials/Neon3.Neon3"))
              (:then_13
                (Rendering|Material|SetMaterial (Variables|Default|GetCube7) 0 "/Game/DemoGame/Materials/Neon3.Neon3"))
              (:then_14
                (Rendering|Material|SetMaterial (Variables|Default|GetCube9) 0 "/Game/DemoGame/Materials/Neon3.Neon3"))
              (:then_15
                (Rendering|Material|SetMaterial (Variables|Default|GetCube10) 0 "/Game/DemoGame/Materials/Neon3.Neon3"))
              (:then_16
                (Rendering|Material|SetMaterial (Variables|Default|GetCube8) 0 "/Game/DemoGame/Materials/Neon3.Neon3")))))))
    (else
      (Variables|Default|SetIs%20open9 false)
      (if (Variables|Default|GetIs%20open9)
        (goto _label)))))

(event OnClicked(Cube4)
  (params (TouchedComponent :type Primitive%20Component%20Object%20Reference) (ButtonPressed :type Key%20Structure :default "None"))
  (Utilities|FlowControl|FlipFlop
    (:A
      (Rendering|Material|SetMaterial (Variables|Default|GetCube4) 0 "/Game/DemoGame/Materials/Neon2.Neon2")
      (Variables|Default|SetTrue1_0 true))
    (:B
      (Rendering|Material|SetMaterial (Variables|Default|GetCube4) 0 "/Game/DemoGame/Materials/Neon.Neon")
      (Variables|Default|SetTrue1_0 false)))
  (if (Variables|Default|GetTrue1_0)
    (Variables|Default|SetIs%20open2 true)
    (if (Variables|Default|GetIs%20open2)
      (if (Math|Boolean|ANDBoolean (Variables|Default|GetIs%20open) (Variables|Default|GetIs%20open2) (Variables|Default|GetIs%20open3) (Variables|Default|GetIs%20open4) (Variables|Default|GetIs%20open5) (Variables|Default|GetIs%20open6) (Variables|Default|GetIs%20open7) (Variables|Default|GetIs%20open8) (Variables|Default|GetIs%20open9) (Variables|Default|GetIs%20open10) (Variables|Default|GetIs%20open11) (Variables|Default|GetIs%20open12)) :!label _label
        (Utilities|FlowControl|DoOnce false
          (:Completed
            (Utilities|FlowControl|Sequence
              (:then_0
                (Rendering|Material|SetMaterial (Variables|Default|GetCube) 1 "/Game/DemoGame/Materials/Neon3.Neon3"))
              (:then_1
                (Rendering|Material|SetMaterial (Variables|Default|GetCube1) 1 "/Game/DemoGame/Materials/Neon3.Neon3"))
              (:then_2
                (Rendering|Material|SetMaterial (Variables|Default|GetCube2) 1 "/Game/DemoGame/Materials/Neon3.Neon3"))
              (:then_3
                (bind _newtrack_0 (Timeline|Timeline Play)
                  (:Update
                    (Transformation|SetRelativeLocation (Variables|/Game/DemoGame/Gates/BP_Third_Gate.BP_Third_Gate_C|GetCube (Variables|Default|GetOpendoor)) (Math|Vector|Lerp(Vector) "0, 0, 0" "0.000000,0.000000,400.000000" _newtrack_0) false false)
                    (Utilities|FlowControl|DoOnce false
                      (:Completed
                        (bind _returnvalue (UserInterface|CreateWidget "/Game/DemoGame/Widgets/WB_Gate_Open.WB_Gate_Open_C"))
                        (UserInterface|Viewport|AddtoViewport _returnvalue 0)
                        (Utilities|FlowControl|Delay 5.0)
                        (Widget|RemovefromParent _returnvalue))))))
              (:then_4
                (Rendering|Material|SetMaterial (Variables|Default|GetCube14) 0 "/Game/DemoGame/Materials/Neon3.Neon3"))
              (:then_5
                (Rendering|Material|SetMaterial (Variables|Default|GetCube13) 0 "/Game/DemoGame/Materials/Neon3.Neon3"))
              (:then_6
                (Rendering|Material|SetMaterial (Variables|Default|GetCube12) 0 "/Game/DemoGame/Materials/Neon3.Neon3"))
              (:then_7
                (Rendering|Material|SetMaterial (Variables|Default|GetCube11) 0 "/Game/DemoGame/Materials/Neon3.Neon3"))
              (:then_8
                (Rendering|Material|SetMaterial (Variables|Default|GetCube6) 0 "/Game/DemoGame/Materials/Neon3.Neon3"))
              (:then_9
                (Rendering|Material|SetMaterial (Variables|Default|GetCube5) 0 "/Game/DemoGame/Materials/Neon3.Neon3"))
              (:then_10
                (Rendering|Material|SetMaterial (Variables|Default|GetCube4) 0 "/Game/DemoGame/Materials/Neon3.Neon3"))
              (:then_11
                (Rendering|Material|SetMaterial (Variables|Default|GetCube3) 0 "/Game/DemoGame/Materials/Neon3.Neon3"))
              (:then_12
                (Rendering|Material|SetMaterial (Variables|Default|GetCube8) 10 "/Game/DemoGame/Materials/Neon3.Neon3"))
              (:then_13
                (Rendering|Material|SetMaterial (Variables|Default|GetCube7) 0 "/Game/DemoGame/Materials/Neon3.Neon3"))
              (:then_14
                (Rendering|Material|SetMaterial (Variables|Default|GetCube9) 0 "/Game/DemoGame/Materials/Neon3.Neon3"))
              (:then_15
                (Rendering|Material|SetMaterial (Variables|Default|GetCube10) 0 "/Game/DemoGame/Materials/Neon3.Neon3"))
              (:then_16
                (Rendering|Material|SetMaterial (Variables|Default|GetCube8) 0 "/Game/DemoGame/Materials/Neon3.Neon3")))))))
    (else
      (Variables|Default|SetIs%20open2 false)
      (if (Variables|Default|GetIs%20open2)
        (goto _label)))))

(event OnClicked(Cube3)
  (params (TouchedComponent :type Primitive%20Component%20Object%20Reference) (ButtonPressed :type Key%20Structure :default "None"))
  (Utilities|FlowControl|FlipFlop
    (:A
      (Rendering|Material|SetMaterial (Variables|Default|GetCube3) 0 "/Game/DemoGame/Materials/Neon2.Neon2")
      (Variables|Default|SetTrue1 true))
    (:B
      (Rendering|Material|SetMaterial (Variables|Default|GetCube3) 0 "/Game/DemoGame/Materials/Neon.Neon")
      (Variables|Default|SetTrue1 false)))
  (if (Variables|Default|GetTrue1)
    (Variables|Default|SetIs%20open true)
    (if (Variables|Default|GetIs%20open)
      (if (Math|Boolean|ANDBoolean (Variables|Default|GetIs%20open) (Variables|Default|GetIs%20open2) (Variables|Default|GetIs%20open3) (Variables|Default|GetIs%20open4) (Variables|Default|GetIs%20open5) (Variables|Default|GetIs%20open6) (Variables|Default|GetIs%20open7) (Variables|Default|GetIs%20open8) (Variables|Default|GetIs%20open9) (Variables|Default|GetIs%20open10) (Variables|Default|GetIs%20open11) (Variables|Default|GetIs%20open12)) :!label _label
        (Utilities|FlowControl|DoOnce false
          (:Completed
            (Utilities|FlowControl|Sequence
              (:then_0
                (Rendering|Material|SetMaterial (Variables|Default|GetCube) 1 "/Game/DemoGame/Materials/Neon3.Neon3"))
              (:then_1
                (Rendering|Material|SetMaterial (Variables|Default|GetCube1) 1 "/Game/DemoGame/Materials/Neon3.Neon3"))
              (:then_2
                (Rendering|Material|SetMaterial (Variables|Default|GetCube2) 1 "/Game/DemoGame/Materials/Neon3.Neon3"))
              (:then_3
                (bind _newtrack_0 (Timeline|Timeline Play)
                  (:Update
                    (Transformation|SetRelativeLocation (Variables|/Game/DemoGame/Gates/BP_Third_Gate.BP_Third_Gate_C|GetCube (Variables|Default|GetOpendoor)) (Math|Vector|Lerp(Vector) "0, 0, 0" "0.000000,0.000000,400.000000" _newtrack_0) false false)
                    (Utilities|FlowControl|DoOnce false
                      (:Completed
                        (bind _returnvalue (UserInterface|CreateWidget "/Game/DemoGame/Widgets/WB_Gate_Open.WB_Gate_Open_C"))
                        (UserInterface|Viewport|AddtoViewport _returnvalue 0)
                        (Utilities|FlowControl|Delay 5.0)
                        (Widget|RemovefromParent _returnvalue))))))
              (:then_4
                (Rendering|Material|SetMaterial (Variables|Default|GetCube14) 0 "/Game/DemoGame/Materials/Neon3.Neon3"))
              (:then_5
                (Rendering|Material|SetMaterial (Variables|Default|GetCube13) 0 "/Game/DemoGame/Materials/Neon3.Neon3"))
              (:then_6
                (Rendering|Material|SetMaterial (Variables|Default|GetCube12) 0 "/Game/DemoGame/Materials/Neon3.Neon3"))
              (:then_7
                (Rendering|Material|SetMaterial (Variables|Default|GetCube11) 0 "/Game/DemoGame/Materials/Neon3.Neon3"))
              (:then_8
                (Rendering|Material|SetMaterial (Variables|Default|GetCube6) 0 "/Game/DemoGame/Materials/Neon3.Neon3"))
              (:then_9
                (Rendering|Material|SetMaterial (Variables|Default|GetCube5) 0 "/Game/DemoGame/Materials/Neon3.Neon3"))
              (:then_10
                (Rendering|Material|SetMaterial (Variables|Default|GetCube4) 0 "/Game/DemoGame/Materials/Neon3.Neon3"))
              (:then_11
                (Rendering|Material|SetMaterial (Variables|Default|GetCube3) 0 "/Game/DemoGame/Materials/Neon3.Neon3"))
              (:then_12
                (Rendering|Material|SetMaterial (Variables|Default|GetCube8) 10 "/Game/DemoGame/Materials/Neon3.Neon3"))
              (:then_13
                (Rendering|Material|SetMaterial (Variables|Default|GetCube7) 0 "/Game/DemoGame/Materials/Neon3.Neon3"))
              (:then_14
                (Rendering|Material|SetMaterial (Variables|Default|GetCube9) 0 "/Game/DemoGame/Materials/Neon3.Neon3"))
              (:then_15
                (Rendering|Material|SetMaterial (Variables|Default|GetCube10) 0 "/Game/DemoGame/Materials/Neon3.Neon3"))
              (:then_16
                (Rendering|Material|SetMaterial (Variables|Default|GetCube8) 0 "/Game/DemoGame/Materials/Neon3.Neon3")))))))
    (else
      (Variables|Default|SetIs%20open false)
      (if (Variables|Default|GetIs%20open)
        (goto _label)))))

(event OnClicked(Cube8)
  (params (TouchedComponent :type Primitive%20Component%20Object%20Reference) (ButtonPressed :type Key%20Structure :default "None"))
  (Utilities|FlowControl|FlipFlop
    (:A
      (Rendering|Material|SetMaterial (Variables|Default|GetCube8) 0 "/Game/DemoGame/Materials/Neon2.Neon2")
      (Variables|Default|SetTrue1_4 false))
    (:B
      (Rendering|Material|SetMaterial (Variables|Default|GetCube8) 0 "/Game/DemoGame/Materials/Neon.Neon")
      (Variables|Default|SetTrue1_4 true)))
  (if (Variables|Default|GetTrue1_4)
    (Variables|Default|SetIs%20open6 true)
    (if (Variables|Default|GetIs%20open6)
      (if (Math|Boolean|ANDBoolean (Variables|Default|GetIs%20open) (Variables|Default|GetIs%20open2) (Variables|Default|GetIs%20open3) (Variables|Default|GetIs%20open4) (Variables|Default|GetIs%20open5) (Variables|Default|GetIs%20open6) (Variables|Default|GetIs%20open7) (Variables|Default|GetIs%20open8) (Variables|Default|GetIs%20open9) (Variables|Default|GetIs%20open10) (Variables|Default|GetIs%20open11) (Variables|Default|GetIs%20open12)) :!label _label
        (Utilities|FlowControl|DoOnce false
          (:Completed
            (Utilities|FlowControl|Sequence
              (:then_0
                (Rendering|Material|SetMaterial (Variables|Default|GetCube) 1 "/Game/DemoGame/Materials/Neon3.Neon3"))
              (:then_1
                (Rendering|Material|SetMaterial (Variables|Default|GetCube1) 1 "/Game/DemoGame/Materials/Neon3.Neon3"))
              (:then_2
                (Rendering|Material|SetMaterial (Variables|Default|GetCube2) 1 "/Game/DemoGame/Materials/Neon3.Neon3"))
              (:then_3
                (bind _newtrack_0 (Timeline|Timeline Play)
                  (:Update
                    (Transformation|SetRelativeLocation (Variables|/Game/DemoGame/Gates/BP_Third_Gate.BP_Third_Gate_C|GetCube (Variables|Default|GetOpendoor)) (Math|Vector|Lerp(Vector) "0, 0, 0" "0.000000,0.000000,400.000000" _newtrack_0) false false)
                    (Utilities|FlowControl|DoOnce false
                      (:Completed
                        (bind _returnvalue (UserInterface|CreateWidget "/Game/DemoGame/Widgets/WB_Gate_Open.WB_Gate_Open_C"))
                        (UserInterface|Viewport|AddtoViewport _returnvalue 0)
                        (Utilities|FlowControl|Delay 5.0)
                        (Widget|RemovefromParent _returnvalue))))))
              (:then_4
                (Rendering|Material|SetMaterial (Variables|Default|GetCube14) 0 "/Game/DemoGame/Materials/Neon3.Neon3"))
              (:then_5
                (Rendering|Material|SetMaterial (Variables|Default|GetCube13) 0 "/Game/DemoGame/Materials/Neon3.Neon3"))
              (:then_6
                (Rendering|Material|SetMaterial (Variables|Default|GetCube12) 0 "/Game/DemoGame/Materials/Neon3.Neon3"))
              (:then_7
                (Rendering|Material|SetMaterial (Variables|Default|GetCube11) 0 "/Game/DemoGame/Materials/Neon3.Neon3"))
              (:then_8
                (Rendering|Material|SetMaterial (Variables|Default|GetCube6) 0 "/Game/DemoGame/Materials/Neon3.Neon3"))
              (:then_9
                (Rendering|Material|SetMaterial (Variables|Default|GetCube5) 0 "/Game/DemoGame/Materials/Neon3.Neon3"))
              (:then_10
                (Rendering|Material|SetMaterial (Variables|Default|GetCube4) 0 "/Game/DemoGame/Materials/Neon3.Neon3"))
              (:then_11
                (Rendering|Material|SetMaterial (Variables|Default|GetCube3) 0 "/Game/DemoGame/Materials/Neon3.Neon3"))
              (:then_12
                (Rendering|Material|SetMaterial (Variables|Default|GetCube8) 10 "/Game/DemoGame/Materials/Neon3.Neon3"))
              (:then_13
                (Rendering|Material|SetMaterial (Variables|Default|GetCube7) 0 "/Game/DemoGame/Materials/Neon3.Neon3"))
              (:then_14
                (Rendering|Material|SetMaterial (Variables|Default|GetCube9) 0 "/Game/DemoGame/Materials/Neon3.Neon3"))
              (:then_15
                (Rendering|Material|SetMaterial (Variables|Default|GetCube10) 0 "/Game/DemoGame/Materials/Neon3.Neon3"))
              (:then_16
                (Rendering|Material|SetMaterial (Variables|Default|GetCube8) 0 "/Game/DemoGame/Materials/Neon3.Neon3")))))))
    (else
      (Variables|Default|SetIs%20open6 false)
      (if (Variables|Default|GetIs%20open6)
        (goto _label)))))

(event OnClicked(Cube7)
  (params (TouchedComponent :type Primitive%20Component%20Object%20Reference) (ButtonPressed :type Key%20Structure :default "None"))
  (Utilities|FlowControl|FlipFlop
    (:A
      (Rendering|Material|SetMaterial (Variables|Default|GetCube7) 0 "/Game/DemoGame/Materials/Neon2.Neon2")
      (Variables|Default|SetTrue1_3 false))
    (:B
      (Rendering|Material|SetMaterial (Variables|Default|GetCube7) 0 "/Game/DemoGame/Materials/Neon.Neon")
      (Variables|Default|SetTrue1_3 true)))
  (if (Variables|Default|GetTrue1_3)
    (Variables|Default|SetIs%20open5 true)
    (if (Variables|Default|GetIs%20open5)
      (if (Math|Boolean|ANDBoolean (Variables|Default|GetIs%20open) (Variables|Default|GetIs%20open2) (Variables|Default|GetIs%20open3) (Variables|Default|GetIs%20open4) (Variables|Default|GetIs%20open5) (Variables|Default|GetIs%20open6) (Variables|Default|GetIs%20open7) (Variables|Default|GetIs%20open8) (Variables|Default|GetIs%20open9) (Variables|Default|GetIs%20open10) (Variables|Default|GetIs%20open11) (Variables|Default|GetIs%20open12)) :!label _label
        (Utilities|FlowControl|DoOnce false
          (:Completed
            (Utilities|FlowControl|Sequence
              (:then_0
                (Rendering|Material|SetMaterial (Variables|Default|GetCube) 1 "/Game/DemoGame/Materials/Neon3.Neon3"))
              (:then_1
                (Rendering|Material|SetMaterial (Variables|Default|GetCube1) 1 "/Game/DemoGame/Materials/Neon3.Neon3"))
              (:then_2
                (Rendering|Material|SetMaterial (Variables|Default|GetCube2) 1 "/Game/DemoGame/Materials/Neon3.Neon3"))
              (:then_3
                (bind _newtrack_0 (Timeline|Timeline Play)
                  (:Update
                    (Transformation|SetRelativeLocation (Variables|/Game/DemoGame/Gates/BP_Third_Gate.BP_Third_Gate_C|GetCube (Variables|Default|GetOpendoor)) (Math|Vector|Lerp(Vector) "0, 0, 0" "0.000000,0.000000,400.000000" _newtrack_0) false false)
                    (Utilities|FlowControl|DoOnce false
                      (:Completed
                        (bind _returnvalue (UserInterface|CreateWidget "/Game/DemoGame/Widgets/WB_Gate_Open.WB_Gate_Open_C"))
                        (UserInterface|Viewport|AddtoViewport _returnvalue 0)
                        (Utilities|FlowControl|Delay 5.0)
                        (Widget|RemovefromParent _returnvalue))))))
              (:then_4
                (Rendering|Material|SetMaterial (Variables|Default|GetCube14) 0 "/Game/DemoGame/Materials/Neon3.Neon3"))
              (:then_5
                (Rendering|Material|SetMaterial (Variables|Default|GetCube13) 0 "/Game/DemoGame/Materials/Neon3.Neon3"))
              (:then_6
                (Rendering|Material|SetMaterial (Variables|Default|GetCube12) 0 "/Game/DemoGame/Materials/Neon3.Neon3"))
              (:then_7
                (Rendering|Material|SetMaterial (Variables|Default|GetCube11) 0 "/Game/DemoGame/Materials/Neon3.Neon3"))
              (:then_8
                (Rendering|Material|SetMaterial (Variables|Default|GetCube6) 0 "/Game/DemoGame/Materials/Neon3.Neon3"))
              (:then_9
                (Rendering|Material|SetMaterial (Variables|Default|GetCube5) 0 "/Game/DemoGame/Materials/Neon3.Neon3"))
              (:then_10
                (Rendering|Material|SetMaterial (Variables|Default|GetCube4) 0 "/Game/DemoGame/Materials/Neon3.Neon3"))
              (:then_11
                (Rendering|Material|SetMaterial (Variables|Default|GetCube3) 0 "/Game/DemoGame/Materials/Neon3.Neon3"))
              (:then_12
                (Rendering|Material|SetMaterial (Variables|Default|GetCube8) 10 "/Game/DemoGame/Materials/Neon3.Neon3"))
              (:then_13
                (Rendering|Material|SetMaterial (Variables|Default|GetCube7) 0 "/Game/DemoGame/Materials/Neon3.Neon3"))
              (:then_14
                (Rendering|Material|SetMaterial (Variables|Default|GetCube9) 0 "/Game/DemoGame/Materials/Neon3.Neon3"))
              (:then_15
                (Rendering|Material|SetMaterial (Variables|Default|GetCube10) 0 "/Game/DemoGame/Materials/Neon3.Neon3"))
              (:then_16
                (Rendering|Material|SetMaterial (Variables|Default|GetCube8) 0 "/Game/DemoGame/Materials/Neon3.Neon3")))))))
    (else
      (Variables|Default|SetIs%20open5 false)
      (if (Variables|Default|GetIs%20open5)
        (goto _label)))))

(event OnClicked(Cube9)
  (params (TouchedComponent :type Primitive%20Component%20Object%20Reference) (ButtonPressed :type Key%20Structure :default "None"))
  (Utilities|FlowControl|FlipFlop
    (:A
      (Rendering|Material|SetMaterial (Variables|Default|GetCube9) 0 "/Game/DemoGame/Materials/Neon2.Neon2")
      (Variables|Default|SetTrue1_5 false))
    (:B
      (Rendering|Material|SetMaterial (Variables|Default|GetCube9) 0 "/Game/DemoGame/Materials/Neon.Neon")
      (Variables|Default|SetTrue1_5 true)))
  (if (Variables|Default|GetTrue1_5)
    (Variables|Default|SetIs%20open7 true)
    (if (Variables|Default|GetIs%20open7)
      (if (Math|Boolean|ANDBoolean (Variables|Default|GetIs%20open) (Variables|Default|GetIs%20open2) (Variables|Default|GetIs%20open3) (Variables|Default|GetIs%20open4) (Variables|Default|GetIs%20open5) (Variables|Default|GetIs%20open6) (Variables|Default|GetIs%20open7) (Variables|Default|GetIs%20open8) (Variables|Default|GetIs%20open9) (Variables|Default|GetIs%20open10) (Variables|Default|GetIs%20open11) (Variables|Default|GetIs%20open12)) :!label _label
        (Utilities|FlowControl|DoOnce false
          (:Completed
            (Utilities|FlowControl|Sequence
              (:then_0
                (Rendering|Material|SetMaterial (Variables|Default|GetCube) 1 "/Game/DemoGame/Materials/Neon3.Neon3"))
              (:then_1
                (Rendering|Material|SetMaterial (Variables|Default|GetCube1) 1 "/Game/DemoGame/Materials/Neon3.Neon3"))
              (:then_2
                (Rendering|Material|SetMaterial (Variables|Default|GetCube2) 1 "/Game/DemoGame/Materials/Neon3.Neon3"))
              (:then_3
                (bind _newtrack_0 (Timeline|Timeline Play)
                  (:Update
                    (Transformation|SetRelativeLocation (Variables|/Game/DemoGame/Gates/BP_Third_Gate.BP_Third_Gate_C|GetCube (Variables|Default|GetOpendoor)) (Math|Vector|Lerp(Vector) "0, 0, 0" "0.000000,0.000000,400.000000" _newtrack_0) false false)
                    (Utilities|FlowControl|DoOnce false
                      (:Completed
                        (bind _returnvalue (UserInterface|CreateWidget "/Game/DemoGame/Widgets/WB_Gate_Open.WB_Gate_Open_C"))
                        (UserInterface|Viewport|AddtoViewport _returnvalue 0)
                        (Utilities|FlowControl|Delay 5.0)
                        (Widget|RemovefromParent _returnvalue))))))
              (:then_4
                (Rendering|Material|SetMaterial (Variables|Default|GetCube14) 0 "/Game/DemoGame/Materials/Neon3.Neon3"))
              (:then_5
                (Rendering|Material|SetMaterial (Variables|Default|GetCube13) 0 "/Game/DemoGame/Materials/Neon3.Neon3"))
              (:then_6
                (Rendering|Material|SetMaterial (Variables|Default|GetCube12) 0 "/Game/DemoGame/Materials/Neon3.Neon3"))
              (:then_7
                (Rendering|Material|SetMaterial (Variables|Default|GetCube11) 0 "/Game/DemoGame/Materials/Neon3.Neon3"))
              (:then_8
                (Rendering|Material|SetMaterial (Variables|Default|GetCube6) 0 "/Game/DemoGame/Materials/Neon3.Neon3"))
              (:then_9
                (Rendering|Material|SetMaterial (Variables|Default|GetCube5) 0 "/Game/DemoGame/Materials/Neon3.Neon3"))
              (:then_10
                (Rendering|Material|SetMaterial (Variables|Default|GetCube4) 0 "/Game/DemoGame/Materials/Neon3.Neon3"))
              (:then_11
                (Rendering|Material|SetMaterial (Variables|Default|GetCube3) 0 "/Game/DemoGame/Materials/Neon3.Neon3"))
              (:then_12
                (Rendering|Material|SetMaterial (Variables|Default|GetCube8) 10 "/Game/DemoGame/Materials/Neon3.Neon3"))
              (:then_13
                (Rendering|Material|SetMaterial (Variables|Default|GetCube7) 0 "/Game/DemoGame/Materials/Neon3.Neon3"))
              (:then_14
                (Rendering|Material|SetMaterial (Variables|Default|GetCube9) 0 "/Game/DemoGame/Materials/Neon3.Neon3"))
              (:then_15
                (Rendering|Material|SetMaterial (Variables|Default|GetCube10) 0 "/Game/DemoGame/Materials/Neon3.Neon3"))
              (:then_16
                (Rendering|Material|SetMaterial (Variables|Default|GetCube8) 0 "/Game/DemoGame/Materials/Neon3.Neon3")))))))
    (else
      (Variables|Default|SetIs%20open7 false)
      (if (Variables|Default|GetIs%20open7)
        (goto _label)))))

(event OnClicked(Cube10)
  (params (TouchedComponent :type Primitive%20Component%20Object%20Reference) (ButtonPressed :type Key%20Structure :default "None"))
  (Utilities|FlowControl|FlipFlop
    (:A
      (Rendering|Material|SetMaterial (Variables|Default|GetCube10) 0 "/Game/DemoGame/Materials/Neon2.Neon2")
      (Variables|Default|SetTrue1_6 true))
    (:B
      (Rendering|Material|SetMaterial (Variables|Default|GetCube10) 0 "/Game/DemoGame/Materials/Neon.Neon")
      (Variables|Default|SetTrue1_6 false)))
  (if (Variables|Default|GetTrue1_6)
    (Variables|Default|SetIs%20open8 true)
    (if (Variables|Default|GetIs%20open8)
      (if (Math|Boolean|ANDBoolean (Variables|Default|GetIs%20open) (Variables|Default|GetIs%20open2) (Variables|Default|GetIs%20open3) (Variables|Default|GetIs%20open4) (Variables|Default|GetIs%20open5) (Variables|Default|GetIs%20open6) (Variables|Default|GetIs%20open7) (Variables|Default|GetIs%20open8) (Variables|Default|GetIs%20open9) (Variables|Default|GetIs%20open10) (Variables|Default|GetIs%20open11) (Variables|Default|GetIs%20open12)) :!label _label
        (Utilities|FlowControl|DoOnce false
          (:Completed
            (Utilities|FlowControl|Sequence
              (:then_0
                (Rendering|Material|SetMaterial (Variables|Default|GetCube) 1 "/Game/DemoGame/Materials/Neon3.Neon3"))
              (:then_1
                (Rendering|Material|SetMaterial (Variables|Default|GetCube1) 1 "/Game/DemoGame/Materials/Neon3.Neon3"))
              (:then_2
                (Rendering|Material|SetMaterial (Variables|Default|GetCube2) 1 "/Game/DemoGame/Materials/Neon3.Neon3"))
              (:then_3
                (bind _newtrack_0 (Timeline|Timeline Play)
                  (:Update
                    (Transformation|SetRelativeLocation (Variables|/Game/DemoGame/Gates/BP_Third_Gate.BP_Third_Gate_C|GetCube (Variables|Default|GetOpendoor)) (Math|Vector|Lerp(Vector) "0, 0, 0" "0.000000,0.000000,400.000000" _newtrack_0) false false)
                    (Utilities|FlowControl|DoOnce false
                      (:Completed
                        (bind _returnvalue (UserInterface|CreateWidget "/Game/DemoGame/Widgets/WB_Gate_Open.WB_Gate_Open_C"))
                        (UserInterface|Viewport|AddtoViewport _returnvalue 0)
                        (Utilities|FlowControl|Delay 5.0)
                        (Widget|RemovefromParent _returnvalue))))))
              (:then_4
                (Rendering|Material|SetMaterial (Variables|Default|GetCube14) 0 "/Game/DemoGame/Materials/Neon3.Neon3"))
              (:then_5
                (Rendering|Material|SetMaterial (Variables|Default|GetCube13) 0 "/Game/DemoGame/Materials/Neon3.Neon3"))
              (:then_6
                (Rendering|Material|SetMaterial (Variables|Default|GetCube12) 0 "/Game/DemoGame/Materials/Neon3.Neon3"))
              (:then_7
                (Rendering|Material|SetMaterial (Variables|Default|GetCube11) 0 "/Game/DemoGame/Materials/Neon3.Neon3"))
              (:then_8
                (Rendering|Material|SetMaterial (Variables|Default|GetCube6) 0 "/Game/DemoGame/Materials/Neon3.Neon3"))
              (:then_9
                (Rendering|Material|SetMaterial (Variables|Default|GetCube5) 0 "/Game/DemoGame/Materials/Neon3.Neon3"))
              (:then_10
                (Rendering|Material|SetMaterial (Variables|Default|GetCube4) 0 "/Game/DemoGame/Materials/Neon3.Neon3"))
              (:then_11
                (Rendering|Material|SetMaterial (Variables|Default|GetCube3) 0 "/Game/DemoGame/Materials/Neon3.Neon3"))
              (:then_12
                (Rendering|Material|SetMaterial (Variables|Default|GetCube8) 10 "/Game/DemoGame/Materials/Neon3.Neon3"))
              (:then_13
                (Rendering|Material|SetMaterial (Variables|Default|GetCube7) 0 "/Game/DemoGame/Materials/Neon3.Neon3"))
              (:then_14
                (Rendering|Material|SetMaterial (Variables|Default|GetCube9) 0 "/Game/DemoGame/Materials/Neon3.Neon3"))
              (:then_15
                (Rendering|Material|SetMaterial (Variables|Default|GetCube10) 0 "/Game/DemoGame/Materials/Neon3.Neon3"))
              (:then_16
                (Rendering|Material|SetMaterial (Variables|Default|GetCube8) 0 "/Game/DemoGame/Materials/Neon3.Neon3")))))))
    (else
      (Variables|Default|SetIs%20open8 false)
      (if (Variables|Default|GetIs%20open8)
        (goto _label)))))

(event OnClicked(Cube14)
  (params (TouchedComponent :type Primitive%20Component%20Object%20Reference) (ButtonPressed :type Key%20Structure :default "None"))
  (Utilities|FlowControl|FlipFlop
    (:A
      (Rendering|Material|SetMaterial (Variables|Default|GetCube14) 0 "/Game/DemoGame/Materials/Neon2.Neon2")
      (Variables|Default|SetTrue1_10 true))
    (:B
      (Rendering|Material|SetMaterial (Variables|Default|GetCube14) 0 "/Game/DemoGame/Materials/Neon.Neon")
      (Variables|Default|SetTrue1_10 false)))
  (if (Variables|Default|GetTrue1_10)
    (Variables|Default|SetIs%20open12 true)
    (if (Variables|Default|GetIs%20open12)
      (if (Math|Boolean|ANDBoolean (Variables|Default|GetIs%20open) (Variables|Default|GetIs%20open2) (Variables|Default|GetIs%20open3) (Variables|Default|GetIs%20open4) (Variables|Default|GetIs%20open5) (Variables|Default|GetIs%20open6) (Variables|Default|GetIs%20open7) (Variables|Default|GetIs%20open8) (Variables|Default|GetIs%20open9) (Variables|Default|GetIs%20open10) (Variables|Default|GetIs%20open11) (Variables|Default|GetIs%20open12)) :!label _label
        (Utilities|FlowControl|DoOnce false
          (:Completed
            (Utilities|FlowControl|Sequence
              (:then_0
                (Rendering|Material|SetMaterial (Variables|Default|GetCube) 1 "/Game/DemoGame/Materials/Neon3.Neon3"))
              (:then_1
                (Rendering|Material|SetMaterial (Variables|Default|GetCube1) 1 "/Game/DemoGame/Materials/Neon3.Neon3"))
              (:then_2
                (Rendering|Material|SetMaterial (Variables|Default|GetCube2) 1 "/Game/DemoGame/Materials/Neon3.Neon3"))
              (:then_3
                (bind _newtrack_0 (Timeline|Timeline Play)
                  (:Update
                    (Transformation|SetRelativeLocation (Variables|/Game/DemoGame/Gates/BP_Third_Gate.BP_Third_Gate_C|GetCube (Variables|Default|GetOpendoor)) (Math|Vector|Lerp(Vector) "0, 0, 0" "0.000000,0.000000,400.000000" _newtrack_0) false false)
                    (Utilities|FlowControl|DoOnce false
                      (:Completed
                        (bind _returnvalue (UserInterface|CreateWidget "/Game/DemoGame/Widgets/WB_Gate_Open.WB_Gate_Open_C"))
                        (UserInterface|Viewport|AddtoViewport _returnvalue 0)
                        (Utilities|FlowControl|Delay 5.0)
                        (Widget|RemovefromParent _returnvalue))))))
              (:then_4
                (Rendering|Material|SetMaterial (Variables|Default|GetCube14) 0 "/Game/DemoGame/Materials/Neon3.Neon3"))
              (:then_5
                (Rendering|Material|SetMaterial (Variables|Default|GetCube13) 0 "/Game/DemoGame/Materials/Neon3.Neon3"))
              (:then_6
                (Rendering|Material|SetMaterial (Variables|Default|GetCube12) 0 "/Game/DemoGame/Materials/Neon3.Neon3"))
              (:then_7
                (Rendering|Material|SetMaterial (Variables|Default|GetCube11) 0 "/Game/DemoGame/Materials/Neon3.Neon3"))
              (:then_8
                (Rendering|Material|SetMaterial (Variables|Default|GetCube6) 0 "/Game/DemoGame/Materials/Neon3.Neon3"))
              (:then_9
                (Rendering|Material|SetMaterial (Variables|Default|GetCube5) 0 "/Game/DemoGame/Materials/Neon3.Neon3"))
              (:then_10
                (Rendering|Material|SetMaterial (Variables|Default|GetCube4) 0 "/Game/DemoGame/Materials/Neon3.Neon3"))
              (:then_11
                (Rendering|Material|SetMaterial (Variables|Default|GetCube3) 0 "/Game/DemoGame/Materials/Neon3.Neon3"))
              (:then_12
                (Rendering|Material|SetMaterial (Variables|Default|GetCube8) 10 "/Game/DemoGame/Materials/Neon3.Neon3"))
              (:then_13
                (Rendering|Material|SetMaterial (Variables|Default|GetCube7) 0 "/Game/DemoGame/Materials/Neon3.Neon3"))
              (:then_14
                (Rendering|Material|SetMaterial (Variables|Default|GetCube9) 0 "/Game/DemoGame/Materials/Neon3.Neon3"))
              (:then_15
                (Rendering|Material|SetMaterial (Variables|Default|GetCube10) 0 "/Game/DemoGame/Materials/Neon3.Neon3"))
              (:then_16
                (Rendering|Material|SetMaterial (Variables|Default|GetCube8) 0 "/Game/DemoGame/Materials/Neon3.Neon3")))))))
    (else
      (Variables|Default|SetIs%20open12 false)
      (if (Variables|Default|GetIs%20open12)
        (goto _label)))))

(event OnClicked(Cube13)
  (params (TouchedComponent :type Primitive%20Component%20Object%20Reference) (ButtonPressed :type Key%20Structure :default "None"))
  (Utilities|FlowControl|FlipFlop
    (:A
      (Rendering|Material|SetMaterial (Variables|Default|GetCube13) 0 "/Game/DemoGame/Materials/Neon2.Neon2")
      (Variables|Default|SetTrue1_9 false))
    (:B
      (Rendering|Material|SetMaterial (Variables|Default|GetCube13) 0 "/Game/DemoGame/Materials/Neon.Neon")
      (Variables|Default|SetTrue1_9 true)))
  (if (Variables|Default|GetTrue1_9)
    (Variables|Default|SetIs%20open11 true)
    (if (Variables|Default|GetIs%20open11)
      (if (Math|Boolean|ANDBoolean (Variables|Default|GetIs%20open) (Variables|Default|GetIs%20open2) (Variables|Default|GetIs%20open3) (Variables|Default|GetIs%20open4) (Variables|Default|GetIs%20open5) (Variables|Default|GetIs%20open6) (Variables|Default|GetIs%20open7) (Variables|Default|GetIs%20open8) (Variables|Default|GetIs%20open9) (Variables|Default|GetIs%20open10) (Variables|Default|GetIs%20open11) (Variables|Default|GetIs%20open12)) :!label _label
        (Utilities|FlowControl|DoOnce false
          (:Completed
            (Utilities|FlowControl|Sequence
              (:then_0
                (Rendering|Material|SetMaterial (Variables|Default|GetCube) 1 "/Game/DemoGame/Materials/Neon3.Neon3"))
              (:then_1
                (Rendering|Material|SetMaterial (Variables|Default|GetCube1) 1 "/Game/DemoGame/Materials/Neon3.Neon3"))
              (:then_2
                (Rendering|Material|SetMaterial (Variables|Default|GetCube2) 1 "/Game/DemoGame/Materials/Neon3.Neon3"))
              (:then_3
                (bind _newtrack_0 (Timeline|Timeline Play)
                  (:Update
                    (Transformation|SetRelativeLocation (Variables|/Game/DemoGame/Gates/BP_Third_Gate.BP_Third_Gate_C|GetCube (Variables|Default|GetOpendoor)) (Math|Vector|Lerp(Vector) "0, 0, 0" "0.000000,0.000000,400.000000" _newtrack_0) false false)
                    (Utilities|FlowControl|DoOnce false
                      (:Completed
                        (bind _returnvalue (UserInterface|CreateWidget "/Game/DemoGame/Widgets/WB_Gate_Open.WB_Gate_Open_C"))
                        (UserInterface|Viewport|AddtoViewport _returnvalue 0)
                        (Utilities|FlowControl|Delay 5.0)
                        (Widget|RemovefromParent _returnvalue))))))
              (:then_4
                (Rendering|Material|SetMaterial (Variables|Default|GetCube14) 0 "/Game/DemoGame/Materials/Neon3.Neon3"))
              (:then_5
                (Rendering|Material|SetMaterial (Variables|Default|GetCube13) 0 "/Game/DemoGame/Materials/Neon3.Neon3"))
              (:then_6
                (Rendering|Material|SetMaterial (Variables|Default|GetCube12) 0 "/Game/DemoGame/Materials/Neon3.Neon3"))
              (:then_7
                (Rendering|Material|SetMaterial (Variables|Default|GetCube11) 0 "/Game/DemoGame/Materials/Neon3.Neon3"))
              (:then_8
                (Rendering|Material|SetMaterial (Variables|Default|GetCube6) 0 "/Game/DemoGame/Materials/Neon3.Neon3"))
              (:then_9
                (Rendering|Material|SetMaterial (Variables|Default|GetCube5) 0 "/Game/DemoGame/Materials/Neon3.Neon3"))
              (:then_10
                (Rendering|Material|SetMaterial (Variables|Default|GetCube4) 0 "/Game/DemoGame/Materials/Neon3.Neon3"))
              (:then_11
                (Rendering|Material|SetMaterial (Variables|Default|GetCube3) 0 "/Game/DemoGame/Materials/Neon3.Neon3"))
              (:then_12
                (Rendering|Material|SetMaterial (Variables|Default|GetCube8) 10 "/Game/DemoGame/Materials/Neon3.Neon3"))
              (:then_13
                (Rendering|Material|SetMaterial (Variables|Default|GetCube7) 0 "/Game/DemoGame/Materials/Neon3.Neon3"))
              (:then_14
                (Rendering|Material|SetMaterial (Variables|Default|GetCube9) 0 "/Game/DemoGame/Materials/Neon3.Neon3"))
              (:then_15
                (Rendering|Material|SetMaterial (Variables|Default|GetCube10) 0 "/Game/DemoGame/Materials/Neon3.Neon3"))
              (:then_16
                (Rendering|Material|SetMaterial (Variables|Default|GetCube8) 0 "/Game/DemoGame/Materials/Neon3.Neon3")))))))
    (else
      (Variables|Default|SetIs%20open11 false)
      (if (Variables|Default|GetIs%20open11)
        (goto _label)))))

(event Input|EnhancedActionEvents|EnhancedInputActionIA_Back
  (params (ActionValue :type Vector%202D%20Structure) (ElapsedSeconds :type Float%20%28double-precision%29) (TriggeredSeconds :type Float%20%28double-precision%29) (InputAction :type Input%20Action%20Object%20Reference :default "/Game/ThirdPerson/Input/Actions/IA_Back.IA_Back"))
  (bind _returnvalue (Game|GetPlayerController 0))
  (:Started
    (Game|Player|SetViewTargetwithBlend _returnvalue (Variables|Default|GetPlayerreff) 0.5 "VTBlend_Linear" 0.0 false)
    (Variables|/Script/Engine.PlayerController|SetbEnableClickEvents _returnvalue false)
    (Variables|/Script/Engine.PlayerController|SetbShowMouseCursor _returnvalue false)
    (Pawn|Components|CharacterMovement|SetMovementMode (Variables|/Script/Engine.Character|GetCharacterMovement (Variables|Default|GetPlayerreff)) "MOVE_Walking" 0)
    (Variables|/Game/ThirdPerson/Blueprints/BP_ThirdPersonCharacter.BP_ThirdPersonCharacter_C|SetCanShoot (Variables|Default|GetPlayerreff) true)
    (Development|PrintString "Out")))

(event EventBeginPlay
  (|CallParentFunction)
  (Input|EnableInput (Game|GetPlayerController 0)))

(event EventInteraction
  (bind _returnvalue (Game|GetPlayerController 0))
  (Game|Player|SetViewTargetwithBlend _returnvalue self 0.5 "VTBlend_Linear" 0.0 false)
  (Variables|/Script/Engine.PlayerController|SetbEnableClickEvents _returnvalue true)
  (Variables|/Script/Engine.PlayerController|SetbShowMouseCursor _returnvalue true)
  (Pawn|Components|CharacterMovement|DisableMovement (Variables|/Script/Engine.Character|GetCharacterMovement (Variables|Default|GetPlayerreff)))
  (Variables|/Game/ThirdPerson/Blueprints/BP_ThirdPersonCharacter.BP_ThirdPersonCharacter_C|SetCanShoot (Variables|Default|GetPlayerreff) false)
  (Development|PrintString "In"))

(fn ConstructionScript
  (|CallParentFunction))