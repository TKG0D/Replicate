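; BP_Console is an interactive puzzle console that opens a gate once all four of its buttons are clicked.
; Interaction blends the camera to the console, enables mouse clicks and locks player movement, while IA_Back restores all three.
; Each clicked cube turns neon and sets a flag, feeding a shared check.
; When all flags are set, the console lights up, a timeline raises Gate1 and a gate-open widget appears temporarily.
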(event OnClicked(Cube1)
  (params (TouchedComponent :type Primitive%20Component%20Object%20Reference) (ButtonPressed :type Key%20Structure :default "None"))
  (Rendering|Material|SetMaterial (Variables|Default|GetCube1) 0 "/Game/DemoGame/Materials/Neon2.Neon2")
  (Utilities|FlowControl|DoOnce false
    (:Completed
      (bind _output_get (Variables|Default|SetButtonGreen true))
      (if (Math|Boolean|ANDBoolean _output_get (stale OnClicked(Cube2) _output_get) (stale OnClicked(Cube3) _output_get) (stale OnClicked(Cube4) _output_get))
        (Variables|Default|SetAllgreen true)
        (if (Variables|Default|GetAllgreen)
          (Rendering|Material|SetMaterial (Variables|Default|GetCube) 1 "/Game/DemoGame/Materials/Neon2.Neon2")
          (Utilities|FlowControl|DoOnce false
            (:Completed
              (bind _newtrack_0 (Timeline|Timeline Play)
                (:Update
                  (Transformation|SetRelativeLocation (Variables|/Game/DemoGame/Gates/BP_Second_Gate.BP_Second_Gate_C|GetCube (Variables|Default|GetGate1)) (Math|Vector|Lerp(Vector) "0, 0, 0" "0.000000,0.000000,1000.000000" _newtrack_0) false false)
                  (Utilities|FlowControl|Delay 2.0)
                  (bind _returnvalue (UserInterface|CreateWidget "/Game/DemoGame/Widgets/WB_Gate_Open.WB_Gate_Open_C"))
                  (UserInterface|Viewport|AddtoViewport _returnvalue 0)
                  (Utilities|FlowControl|Delay 5.0)
                  (Widget|RemovefromParent _returnvalue))))))))))

(event OnClicked(Cube2)
  (params (TouchedComponent :type Primitive%20Component%20Object%20Reference) (ButtonPressed :type Key%20Structure :default "None"))
  (Rendering|Material|SetMaterial (Variables|Default|GetCube2) 0 "/Game/DemoGame/Materials/Neon2.Neon2")
  (Utilities|FlowControl|DoOnce false
    (:Completed
      (bind _output_get (Variables|Default|SetButtonGreen2 true))
      (if (Math|Boolean|ANDBoolean (stale OnClicked(Cube1) _output_get) _output_get (stale OnClicked(Cube3) _output_get) (stale OnClicked(Cube4) _output_get))
        (Variables|Default|SetAllgreen true)
        (if (Variables|Default|GetAllgreen)
          (Rendering|Material|SetMaterial (Variables|Default|GetCube) 1 "/Game/DemoGame/Materials/Neon2.Neon2")
          (Utilities|FlowControl|DoOnce false
            (:Completed
              (bind _newtrack_0 (Timeline|Timeline Play)
                (:Update
                  (Transformation|SetRelativeLocation (Variables|/Game/DemoGame/Gates/BP_Second_Gate.BP_Second_Gate_C|GetCube (Variables|Default|GetGate1)) (Math|Vector|Lerp(Vector) "0, 0, 0" "0.000000,0.000000,1000.000000" _newtrack_0) false false)
                  (Utilities|FlowControl|Delay 2.0)
                  (bind _returnvalue (UserInterface|CreateWidget "/Game/DemoGame/Widgets/WB_Gate_Open.WB_Gate_Open_C"))
                  (UserInterface|Viewport|AddtoViewport _returnvalue 0)
                  (Utilities|FlowControl|Delay 5.0)
                  (Widget|RemovefromParent _returnvalue))))))))))

(event OnClicked(Cube3)
  (params (TouchedComponent :type Primitive%20Component%20Object%20Reference) (ButtonPressed :type Key%20Structure :default "None"))
  (Rendering|Material|SetMaterial (Variables|Default|GetCube3) 0 "/Game/DemoGame/Materials/Neon2.Neon2")
  (Utilities|FlowControl|DoOnce false
    (:Completed
      (bind _output_get (Variables|Default|SetButtonGreen3 true))
      (if (Math|Boolean|ANDBoolean (stale OnClicked(Cube1) _output_get) (stale OnClicked(Cube2) _output_get) _output_get (stale OnClicked(Cube4) _output_get))
        (Variables|Default|SetAllgreen true)
        (if (Variables|Default|GetAllgreen)
          (Rendering|Material|SetMaterial (Variables|Default|GetCube) 1 "/Game/DemoGame/Materials/Neon2.Neon2")
          (Utilities|FlowControl|DoOnce false
            (:Completed
              (bind _newtrack_0 (Timeline|Timeline Play)
                (:Update
                  (Transformation|SetRelativeLocation (Variables|/Game/DemoGame/Gates/BP_Second_Gate.BP_Second_Gate_C|GetCube (Variables|Default|GetGate1)) (Math|Vector|Lerp(Vector) "0, 0, 0" "0.000000,0.000000,1000.000000" _newtrack_0) false false)
                  (Utilities|FlowControl|Delay 2.0)
                  (bind _returnvalue (UserInterface|CreateWidget "/Game/DemoGame/Widgets/WB_Gate_Open.WB_Gate_Open_C"))
                  (UserInterface|Viewport|AddtoViewport _returnvalue 0)
                  (Utilities|FlowControl|Delay 5.0)
                  (Widget|RemovefromParent _returnvalue))))))))))

(event OnClicked(Cube4)
  (params (TouchedComponent :type Primitive%20Component%20Object%20Reference) (ButtonPressed :type Key%20Structure :default "None"))
  (Rendering|Material|SetMaterial (Variables|Default|GetCube4) 0 "/Game/DemoGame/Materials/Neon2.Neon2")
  (Utilities|FlowControl|DoOnce false
    (:Completed
      (bind _output_get (Variables|Default|SetButtonGreen4 true))
      (if (Math|Boolean|ANDBoolean (stale OnClicked(Cube1) _output_get) (stale OnClicked(Cube2) _output_get) (stale OnClicked(Cube3) _output_get) _output_get)
        (Variables|Default|SetAllgreen true)
        (if (Variables|Default|GetAllgreen)
          (Rendering|Material|SetMaterial (Variables|Default|GetCube) 1 "/Game/DemoGame/Materials/Neon2.Neon2")
          (Utilities|FlowControl|DoOnce false
            (:Completed
              (bind _newtrack_0 (Timeline|Timeline Play)
                (:Update
                  (Transformation|SetRelativeLocation (Variables|/Game/DemoGame/Gates/BP_Second_Gate.BP_Second_Gate_C|GetCube (Variables|Default|GetGate1)) (Math|Vector|Lerp(Vector) "0, 0, 0" "0.000000,0.000000,1000.000000" _newtrack_0) false false)
                  (Utilities|FlowControl|Delay 2.0)
                  (bind _returnvalue (UserInterface|CreateWidget "/Game/DemoGame/Widgets/WB_Gate_Open.WB_Gate_Open_C"))
                  (UserInterface|Viewport|AddtoViewport _returnvalue 0)
                  (Utilities|FlowControl|Delay 5.0)
                  (Widget|RemovefromParent _returnvalue))))))))))

(event Input|EnhancedActionEvents|EnhancedInputActionIA_Back
  (params (ActionValue :type Vector%202D%20Structure) (ElapsedSeconds :type Float%20%28double-precision%29) (TriggeredSeconds :type Float%20%28double-precision%29) (InputAction :type Input%20Action%20Object%20Reference :default "/Game/ThirdPerson/Input/Actions/IA_Back.IA_Back"))
  (bind _returnvalue (Game|GetPlayerController 0))
  (:Started
    (Game|Player|SetViewTargetwithBlend _returnvalue (Variables|Default|GetPlayerreff) 0.5 "VTBlend_Linear" 0.0 false)
    (Variables|/Script/Engine.PlayerController|SetbEnableClickEvents _returnvalue false)
    (Variables|/Script/Engine.PlayerController|SetbShowMouseCursor _returnvalue false)
    (Pawn|Components|CharacterMovement|SetMovementMode (Variables|/Script/Engine.Character|GetCharacterMovement (Variables|Default|GetPlayerreff)) "MOVE_Walking" 0)))

(event EventBeginPlay
  (|CallParentFunction)
  (Input|EnableInput (Game|GetPlayerController 0)))

(event EventInteraction
  (bind _returnvalue (Game|GetPlayerController 0))
  (Game|Player|SetViewTargetwithBlend _returnvalue self 0.5 "VTBlend_Linear" 0.0 false)
  (Variables|/Script/Engine.PlayerController|SetbEnableClickEvents _returnvalue true)
  (Variables|/Script/Engine.PlayerController|SetbShowMouseCursor _returnvalue true)
  (Pawn|Components|CharacterMovement|DisableMovement (Variables|/Script/Engine.Character|GetCharacterMovement (Variables|Default|GetPlayerreff))))

(fn ConstructionScript
  (|CallParentFunction))

(fn NewFunction)