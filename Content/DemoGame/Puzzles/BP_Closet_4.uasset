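; BP_Closet_4 is a four-switch puzzle closet that sets OpenElectricity3 when solved.
; Interaction blends the view to the closet, enables mouse clicks and stops player movement; IA_Back restores both view and movement.
; Each switch flip-flops between two neon materials and its Open flag, with 1 and 4 true on Neon, 2 and 3 on Neon2.
; When all four flags are true, a DoOnce turns the cube and switches Neon2.
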(event OnClicked(2)
  (params (TouchedComponent :type Primitive%20Component%20Object%20Reference) (ButtonPressed :type Key%20Structure :default "None"))
  (Utilities|FlowControl|FlipFlop
    (:A
      (Rendering|Material|SetMaterial (Variables|Default|Get2) 0 "/Game/DemoGame/Materials/Neon.Neon")
      (Variables|Default|SetTrue2 false))
    (:B
      (Rendering|Material|SetMaterial (Variables|Default|Get2) 0 "/Game/DemoGame/Materials/Neon2.Neon2")
      (Variables|Default|SetTrue2 true)))
  (if (Variables|Default|GetTrue2)
    (Variables|Default|SetOpen2 true)
    (if (Variables|Default|GetOpen2)
      (if (Math|Boolean|ANDBoolean (Variables|Default|GetOpen1) (Variables|Default|GetOpen2) (Variables|Default|GetOpen3) (Variables|Default|GetOpen4)) :!label _label
        (Utilities|FlowControl|DoOnce false
          (:Completed
            (Utilities|FlowControl|Sequence
              (:then_0
                (Rendering|Material|SetMaterial (Variables|Default|GetCube) 0 "/Game/DemoGame/Materials/Neon2.Neon2")
                (bind _output_get (Variables|Default|SetOpen%20Electricity3 true))
                (Development|PrintString (Utilities|String|ToString(Boolean) _output_get)))
              (:then_1
                (Rendering|Material|SetMaterial (Variables|Default|GetCube) 1 "/Game/DemoGame/Materials/Neon2.Neon2"))
              (:then_2
                (Rendering|Material|SetMaterial (Variables|Default|Get2) 0 "/Game/DemoGame/Materials/Neon2.Neon2"))
              (:then_3
                (Rendering|Material|SetMaterial (Variables|Default|Get1) 0 "/Game/DemoGame/Materials/Neon2.Neon2"))
              (:then_4
                (Rendering|Material|SetMaterial (Variables|Default|Get3) 0 "/Game/DemoGame/Materials/Neon2.Neon2"))
              (:then_5
                (Rendering|Material|SetMaterial (Variables|Default|Get4) 0 "/Game/DemoGame/Materials/Neon2.Neon2")))))))
    (else
      (Variables|Default|SetOpen2 false)
      (if (Variables|Default|GetOpen2)
        (goto _label)))))

(event OnClicked(1)
  (params (TouchedComponent :type Primitive%20Component%20Object%20Reference) (ButtonPressed :type Key%20Structure :default "None"))
  (Utilities|FlowControl|FlipFlop
    (:A
      (Rendering|Material|SetMaterial (Variables|Default|Get1) 0 "/Game/DemoGame/Materials/Neon.Neon")
      (Variables|Default|SetTrue1 true))
    (:B
      (Rendering|Material|SetMaterial (Variables|Default|Get1) 0 "/Game/DemoGame/Materials/Neon2.Neon2")
      (Variables|Default|SetTrue1 false)))
  (if (Variables|Default|GetTrue1)
    (Variables|Default|SetOpen1 true)
    (if (Variables|Default|GetOpen1)
      (if (Math|Boolean|ANDBoolean (Variables|Default|GetOpen1) (Variables|Default|GetOpen2) (Variables|Default|GetOpen3) (Variables|Default|GetOpen4)) :!label _label
        (Utilities|FlowControl|DoOnce false
          (:Completed
            (Utilities|FlowControl|Sequence
              (:then_0
                (Rendering|Material|SetMaterial (Variables|Default|GetCube) 0 "/Game/DemoGame/Materials/Neon2.Neon2")
                (bind _output_get (Variables|Default|SetOpen%20Electricity3 true))
                (Development|PrintString (Utilities|String|ToString(Boolean) _output_get)))
              (:then_1
                (Rendering|Material|SetMaterial (Variables|Default|GetCube) 1 "/Game/DemoGame/Materials/Neon2.Neon2"))
              (:then_2
                (Rendering|Material|SetMaterial (Variables|Default|Get2) 0 "/Game/DemoGame/Materials/Neon2.Neon2"))
              (:then_3
                (Rendering|Material|SetMaterial (Variables|Default|Get1) 0 "/Game/DemoGame/Materials/Neon2.Neon2"))
              (:then_4
                (Rendering|Material|SetMaterial (Variables|Default|Get3) 0 "/Game/DemoGame/Materials/Neon2.Neon2"))
              (:then_5
                (Rendering|Material|SetMaterial (Variables|Default|Get4) 0 "/Game/DemoGame/Materials/Neon2.Neon2")))))))
    (else
      (Variables|Default|SetOpen1 false)
      (if (Variables|Default|GetOpen1)
        (goto _label)))))

(event OnClicked(3)
  (params (TouchedComponent :type Primitive%20Component%20Object%20Reference) (ButtonPressed :type Key%20Structure :default "None"))
  (Utilities|FlowControl|FlipFlop
    (:A
      (Rendering|Material|SetMaterial (Variables|Default|Get3) 0 "/Game/DemoGame/Materials/Neon.Neon")
      (Variables|Default|SetTrue3 false))
    (:B
      (Rendering|Material|SetMaterial (Variables|Default|Get3) 0 "/Game/DemoGame/Materials/Neon2.Neon2")
      (Variables|Default|SetTrue3 true)))
  (if (Variables|Default|GetTrue3)
    (Variables|Default|SetOpen3 true)
    (if (Variables|Default|GetOpen3)
      (if (Math|Boolean|ANDBoolean (Variables|Default|GetOpen1) (Variables|Default|GetOpen2) (Variables|Default|GetOpen3) (Variables|Default|GetOpen4)) :!label _label
        (Utilities|FlowControl|DoOnce false
          (:Completed
            (Utilities|FlowControl|Sequence
              (:then_0
                (Rendering|Material|SetMaterial (Variables|Default|GetCube) 0 "/Game/DemoGame/Materials/Neon2.Neon2")
                (bind _output_get (Variables|Default|SetOpen%20Electricity3 true))
                (Development|PrintString (Utilities|String|ToString(Boolean) _output_get)))
              (:then_1
                (Rendering|Material|SetMaterial (Variables|Default|GetCube) 1 "/Game/DemoGame/Materials/Neon2.Neon2"))
              (:then_2
                (Rendering|Material|SetMaterial (Variables|Default|Get2) 0 "/Game/DemoGame/Materials/Neon2.Neon2"))
              (:then_3
                (Rendering|Material|SetMaterial (Variables|Default|Get1) 0 "/Game/DemoGame/Materials/Neon2.Neon2"))
              (:then_4
                (Rendering|Material|SetMaterial (Variables|Default|Get3) 0 "/Game/DemoGame/Materials/Neon2.Neon2"))
              (:then_5
                (Rendering|Material|SetMaterial (Variables|Default|Get4) 0 "/Game/DemoGame/Materials/Neon2.Neon2")))))))
    (else
      (Variables|Default|SetOpen3 false)
      (if (Variables|Default|GetOpen3)
        (goto _label)))))

(event OnClicked(4)
  (params (TouchedComponent :type Primitive%20Component%20Object%20Reference) (ButtonPressed :type Key%20Structure :default "None"))
  (Utilities|FlowControl|FlipFlop
    (:A
      (Rendering|Material|SetMaterial (Variables|Default|Get4) 0 "/Game/DemoGame/Materials/Neon.Neon")
      (Variables|Default|SetTrue4 true))
    (:B
      (Rendering|Material|SetMaterial (Variables|Default|Get4) 0 "/Game/DemoGame/Materials/Neon2.Neon2")
      (Variables|Default|SetTrue4 false)))
  (if (Variables|Default|GetTrue4)
    (Variables|Default|SetOpen4 true)
    (if (Variables|Default|GetOpen4)
      (if (Math|Boolean|ANDBoolean (Variables|Default|GetOpen1) (Variables|Default|GetOpen2) (Variables|Default|GetOpen3) (Variables|Default|GetOpen4)) :!label _label
        (Utilities|FlowControl|DoOnce false
          (:Completed
            (Utilities|FlowControl|Sequence
              (:then_0
                (Rendering|Material|SetMaterial (Variables|Default|GetCube) 0 "/Game/DemoGame/Materials/Neon2.Neon2")
                (bind _output_get (Variables|Default|SetOpen%20Electricity3 true))
                (Development|PrintString (Utilities|String|ToString(Boolean) _output_get)))
              (:then_1
                (Rendering|Material|SetMaterial (Variables|Default|GetCube) 1 "/Game/DemoGame/Materials/Neon2.Neon2"))
              (:then_2
                (Rendering|Material|SetMaterial (Variables|Default|Get2) 0 "/Game/DemoGame/Materials/Neon2.Neon2"))
              (:then_3
                (Rendering|Material|SetMaterial (Variables|Default|Get1) 0 "/Game/DemoGame/Materials/Neon2.Neon2"))
              (:then_4
                (Rendering|Material|SetMaterial (Variables|Default|Get3) 0 "/Game/DemoGame/Materials/Neon2.Neon2"))
              (:then_5
                (Rendering|Material|SetMaterial (Variables|Default|Get4) 0 "/Game/DemoGame/Materials/Neon2.Neon2")))))))
    (else
      (Variables|Default|SetOpen4 false)
      (if (Variables|Default|GetOpen4)
        (goto _label)))))

(event Input|EnhancedActionEvents|EnhancedInputActionIA_Back
  (params (ActionValue :type Vector%202D%20Structure) (ElapsedSeconds :type Float%20%28double-precision%29) (TriggeredSeconds :type Float%20%28double-precision%29) (InputAction :type Input%20Action%20Object%20Reference :default "/Game/ThirdPerson/Input/Actions/IA_Back.IA_Back"))
  (bind _returnvalue (Game|GetPlayerController 0))
  (:Started
    (Game|Player|SetViewTargetwithBlend _returnvalue (Variables|Default|GetPlayerreff) 0.5 "VTBlend_Linear" 0.0 false)
    (Variables|/Script/Engine.PlayerController|SetbEnableClickEvents _returnvalue false)
    (Variables|/Script/Engine.PlayerController|SetbShowMouseCursor _returnvalue false)
    (Pawn|Components|CharacterMovement|SetMovementMode (Variables|/Script/Engine.Character|GetCharacterMovement (Variables|Default|GetPlayerreff)) "MOVE_Walking" 0)))

(event EventBeginPlay
  (|CallParentFunction)
  (Input|EnableInput (Game|GetPlayerController 0)))

(event EventInteraction
  (bind _returnvalue (Game|GetPlayerController 0))
  (Game|Player|SetViewTargetwithBlend _returnvalue self 0.5 "VTBlend_Linear" 0.0 false)
  (Variables|/Script/Engine.PlayerController|SetbEnableClickEvents _returnvalue true)
  (Variables|/Script/Engine.PlayerController|SetbShowMouseCursor _returnvalue true)
  (Pawn|Components|CharacterMovement|DisableMovement (Variables|/Script/Engine.Character|GetCharacterMovement (Variables|Default|GetPlayerreff))))

(event EventTick
  (params (DeltaSeconds :type Float%20%28single-precision%29)))

(event Collision|EventActorBeginOverlap
  (params (OtherActor :type Actor%20Object%20Reference)))

(fn ConstructionScript)