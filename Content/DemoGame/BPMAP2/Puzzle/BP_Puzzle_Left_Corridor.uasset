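; Left corridor puzzle actor with four clickable meshes that open a linked door when all are switched on.
; Interaction blends the view to the puzzle, enables mouse clicks and disables player movement and shooting; IA_Back restores them.
; Each click flip-flops a mesh's neon material and its flag.
; With all four flags set, a DoOnce changes the Cube material and plays a Timeline lowering the door's mesh.
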(event OnClicked(Cube1)
  (params (TouchedComponent :type Primitive%20Component%20Object%20Reference) (ButtonPressed :type Key%20Structure))
  (Utilities|FlowControl|FlipFlop
    (:A
      (Rendering|Material|SetMaterial (Variables|Default|GetCube1) 0 "/Game/DemoGame/Materials/Neon.Neon")
      (Development|PrintString "True")
      (Variables|Default|SetTrue true))
    (:B
      (Rendering|Material|SetMaterial (Variables|Default|GetCube1) 0 "/Game/DemoGame/Materials/Neon2.Neon2")
      (Development|PrintString "True")
      (Variables|Default|SetTrue false)))
  (if (Variables|Default|GetTrue)
    (Variables|Default|SetOpen true)
    (if (Variables|Default|GetOpen)
      (if (Math|Boolean|ANDBoolean (Variables|Default|GetOpen_0) (Variables|Default|GetOpen) (Variables|Default|GetOpen_1) (Variables|Default|GetOpen_2)) :!label _label
        (Utilities|FlowControl|DoOnce false
          (:Completed
            (Rendering|Material|SetMaterial (Variables|Default|GetCube) 1 "/Game/DemoGame/Materials/Neon.Neon")
            (Development|PrintString "Hello")
            (bind _newtrack_0 (Timeline|Timeline Play)
              (:Update
                (Transformation|SetRelativeLocation (Variables|/Game/DemoGame/BPMAP2/Doors/BP_Left_Corridor.BP_Left_Corridor_C|GetCube (Variables|Default|GetDoor)) (Math|Vector|Lerp(Vector) "0, 0, 0" "0.000000,0.000000,-750.000000" _newtrack_0) false false)))))))
    (else
      (Variables|Default|SetOpen false)
      (if (Variables|Default|GetOpen)
        (goto _label)))))

(event OnClicked(Cube2)
  (params (TouchedComponent :type Primitive%20Component%20Object%20Reference) (ButtonPressed :type Key%20Structure))
  (Utilities|FlowControl|FlipFlop
    (:A
      (Rendering|Material|SetMaterial (Variables|Default|GetCube2) 0 "/Game/DemoGame/Materials/Neon.Neon")
      (Development|PrintString "True")
      (Variables|Default|SetTrue_0 true))
    (:B
      (Rendering|Material|SetMaterial (Variables|Default|GetCube2) 0 "/Game/DemoGame/Materials/Neon2.Neon2")
      (Development|PrintString "True")
      (Variables|Default|SetTrue_0 false)))
  (if (Variables|Default|GetTrue_0)
    (Variables|Default|SetOpen_0 true)
    (if (Variables|Default|GetOpen_0)
      (if (Math|Boolean|ANDBoolean (Variables|Default|GetOpen_0) (Variables|Default|GetOpen) (Variables|Default|GetOpen_1) (Variables|Default|GetOpen_2)) :!label _label
        (Utilities|FlowControl|DoOnce false
          (:Completed
            (Rendering|Material|SetMaterial (Variables|Default|GetCube) 1 "/Game/DemoGame/Materials/Neon.Neon")
            (Development|PrintString "Hello")
            (bind _newtrack_0 (Timeline|Timeline Play)
              (:Update
                (Transformation|SetRelativeLocation (Variables|/Game/DemoGame/BPMAP2/Doors/BP_Left_Corridor.BP_Left_Corridor_C|GetCube (Variables|Default|GetDoor)) (Math|Vector|Lerp(Vector) "0, 0, 0" "0.000000,0.000000,-750.000000" _newtrack_0) false false)))))))
    (else
      (Variables|Default|SetOpen_0 false)
      (if (Variables|Default|GetOpen_0)
        (goto _label)))))

(event OnClicked(StaticMesh)
  (params (TouchedComponent :type Primitive%20Component%20Object%20Reference) (ButtonPressed :type Key%20Structure))
  (Utilities|FlowControl|FlipFlop
    (:A
      (Rendering|Material|SetMaterial (Variables|Default|GetStaticMesh) 0 "/Game/DemoGame/Materials/Neon.Neon")
      (Development|PrintString "True")
      (Variables|Default|SetTrue_1 true))
    (:B
      (Rendering|Material|SetMaterial (Variables|Default|GetStaticMesh) 0 "/Game/DemoGame/Materials/Neon2.Neon2")
      (Development|PrintString "True")
      (Variables|Default|SetTrue_1 false)))
  (if (Variables|Default|GetTrue_1)
    (Variables|Default|SetOpen_1 true)
    (if (Variables|Default|GetOpen_1)
      (if (Math|Boolean|ANDBoolean (Variables|Default|GetOpen_0) (Variables|Default|GetOpen) (Variables|Default|GetOpen_1) (Variables|Default|GetOpen_2)) :!label _label
        (Utilities|FlowControl|DoOnce false
          (:Completed
            (Rendering|Material|SetMaterial (Variables|Default|GetCube) 1 "/Game/DemoGame/Materials/Neon.Neon")
            (Development|PrintString "Hello")
            (bind _newtrack_0 (Timeline|Timeline Play)
              (:Update
                (Transformation|SetRelativeLocation (Variables|/Game/DemoGame/BPMAP2/Doors/BP_Left_Corridor.BP_Left_Corridor_C|GetCube (Variables|Default|GetDoor)) (Math|Vector|Lerp(Vector) "0, 0, 0" "0.000000,0.000000,-750.000000" _newtrack_0) false false)))))))
    (else
      (Variables|Default|SetOpen_1 false)
      (if (Variables|Default|GetOpen_1)
        (goto _label)))))

(event OnClicked(StaticMesh1)
  (params (TouchedComponent :type Primitive%20Component%20Object%20Reference) (ButtonPressed :type Key%20Structure))
  (Utilities|FlowControl|FlipFlop
    (:A
      (Rendering|Material|SetMaterial (Variables|Default|GetStaticMesh1) 0 "/Game/DemoGame/Materials/Neon.Neon")
      (Development|PrintString "True")
      (Variables|Default|SetTrue_2 true))
    (:B
      (Rendering|Material|SetMaterial (Variables|Default|GetStaticMesh1) 0 "/Game/DemoGame/Materials/Neon2.Neon2")
      (Development|PrintString "True")
      (Variables|Default|SetTrue_2 false)))
  (if (Variables|Default|GetTrue_2)
    (Variables|Default|SetOpen_2 true)
    (if (Variables|Default|GetOpen_2)
      (if (Math|Boolean|ANDBoolean (Variables|Default|GetOpen_0) (Variables|Default|GetOpen) (Variables|Default|GetOpen_1) (Variables|Default|GetOpen_2)) :!label _label
        (Utilities|FlowControl|DoOnce false
          (:Completed
            (Rendering|Material|SetMaterial (Variables|Default|GetCube) 1 "/Game/DemoGame/Materials/Neon.Neon")
            (Development|PrintString "Hello")
            (bind _newtrack_0 (Timeline|Timeline Play)
              (:Update
                (Transformation|SetRelativeLocation (Variables|/Game/DemoGame/BPMAP2/Doors/BP_Left_Corridor.BP_Left_Corridor_C|GetCube (Variables|Default|GetDoor)) (Math|Vector|Lerp(Vector) "0, 0, 0" "0.000000,0.000000,-750.000000" _newtrack_0) false false)))))))
    (else
      (Variables|Default|SetOpen_2 false)
      (if (Variables|Default|GetOpen_2)
        (goto _label)))))

(event Input|EnhancedActionEvents|EnhancedInputActionIA_Back
  (params (ActionValue :type Vector%202D%20Structure) (ElapsedSeconds :type Float%20%28double-precision%29) (TriggeredSeconds :type Float%20%28double-precision%29) (InputAction :type Input%20Action%20Object%20Reference :default "/Game/ThirdPerson/Input/Actions/IA_Back.IA_Back"))
  (bind _returnvalue (Game|GetPlayerController 0))
  (:Started
    (Game|Player|SetViewTargetwithBlend _returnvalue (Variables|Default|GetPlayerreff) 0.5 "VTBlend_Linear" 0.0 false)
    (Variables|/Script/Engine.PlayerController|SetbEnableClickEvents _returnvalue false)
    (Variables|/Script/Engine.PlayerController|SetbShowMouseCursor _returnvalue false)
    (Pawn|Components|CharacterMovement|SetMovementMode (Variables|/Script/Engine.Character|GetCharacterMovement (Variables|Default|GetPlayerreff)) "MOVE_Walking" 0)
    (Variables|/Game/ThirdPerson/Blueprints/BP_ThirdPersonCharacter.BP_ThirdPersonCharacter_C|SetCanShoot (Variables|Default|GetPlayerreff) true)))

(event EventBeginPlay
  (|CallParentFunction)
  (Input|EnableInput (Game|GetPlayerController 0)))

(event EventInteraction
  (bind _returnvalue (Game|GetPlayerController 0))
  (Game|Player|SetViewTargetwithBlend _returnvalue self 0.5 "VTBlend_Linear" 0.0 false)
  (Variables|/Script/Engine.PlayerController|SetbEnableClickEvents _returnvalue true)
  (Variables|/Script/Engine.PlayerController|SetbShowMouseCursor _returnvalue true)
  (Pawn|Components|CharacterMovement|DisableMovement (Variables|/Script/Engine.Character|GetCharacterMovement (Variables|Default|GetPlayerreff)))
  (Variables|/Game/ThirdPerson/Blueprints/BP_ThirdPersonCharacter.BP_ThirdPersonCharacter_C|SetCanShoot (Variables|Default|GetPlayerreff) false))

(event EventTick
  (params (DeltaSeconds :type Float%20%28single-precision%29))
  (|CallParentFunction DeltaSeconds) ; This node is disabled and will not be called.\nDrag off pins to build functionality.
)

(event Collision|EventActorBeginOverlap
  (params (OtherActor :type Actor%20Object%20Reference))
  (|CallParentFunction OtherActor) ; This node is disabled and will not be called.\nDrag off pins to build functionality.
)

(fn ConstructionScript
  (|CallParentFunction))