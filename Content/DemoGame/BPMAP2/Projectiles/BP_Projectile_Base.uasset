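; Base projectile actor that flies via a ProjectileMovement component and is destroyed on impact.
; The construction script copies its Speed and Gravity variables into the movement component, with Speed setting both initial and max speed.
; When the Box component registers a hit, it fires the OnprojectileImpact dispatcher with the hit actor and result, spawns ImpactEffect at the hit location, then destroys itself.
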(event OnComponentHit(Box)
  (params (HitComponent :type Primitive%20Component%20Object%20Reference) (OtherActor :type Actor%20Object%20Reference) (OtherComp :type Primitive%20Component%20Object%20Reference) (NormalImpulse :type Vector :default "0, 0, 0") (Hit :type Hit%20Result%20Structure%20%28by%20ref%29))
  (Default|CallOnprojectileImpact OtherActor Hit)
  (Effects|SpawnEmitteratLocation (Variables|Effects|GetImpact%20Effect) (.Location (Collision|BreakHitResult Hit)))
  (Actor|DestroyActor))

(fn ConstructionScript
  (bind _projectilemovement (Variables|Default|GetProjectileMovement))
  (Variables|/Script/Engine.ProjectileMovementComponent|SetInitialSpeed _projectilemovement (Variables|PorjectileSettings|GetSpeed))
  (Variables|/Script/Engine.ProjectileMovementComponent|SetMaxSpeed _projectilemovement (Variables|PorjectileSettings|GetSpeed))
  (Variables|/Script/Engine.ProjectileMovementComponent|SetProjectileGravityScale _projectilemovement (Variables|PorjectileSettings|GetGravity)))