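; Stun projectile that triggers a state change on specific trap, platform and enemy actors it hits.
; On a Box component hit, a Sequence tries a separate cast for each supported class.
; Turning platform, mid laser and both rotating blade types get their turning flag set and a Start-type function called.
; The spinning piston only gets its flag set, while Enemy 1 receives a Stop call.
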(event OnComponentHit(Box)
  (params (HitComponent :type Primitive%20Component%20Object%20Reference) (OtherActor :type Actor%20Object%20Reference) (OtherComp :type Primitive%20Component%20Object%20Reference) (NormalImpulse :type Vector :default "0, 0, 0") (Hit :type Hit%20Result%20Structure%20%28by%20ref%29))
  (Utilities|FlowControl|Sequence
    (:then_0
      (bind _asbp_turning_platform (Utilities|Casting|CastToBP_Turning_Platform OtherActor))
      (Variables|/Game/BP_Turning_Platform.BP_Turning_Platform_C|SetIsTurningTrue _asbp_turning_platform true)
      (Default|Start _asbp_turning_platform))
    (:then_1
      (bind _asbp_laser_mid (Utilities|Casting|CastToBP_Laser_Mid OtherActor))
      (Variables|/Game/DemoGame/BPMAP2/Traps/BP_Laser_Mid.BP_Laser_Mid_C|SetIsturning _asbp_laser_mid true)
      (Default|Start2 _asbp_laser_mid))
    (:then_2
      (bind _asbp_spinning_piston (Utilities|Casting|CastToBP_Spinning_Piston OtherActor))
      (Variables|/Game/DemoGame/BPMAP2/Traps/BP_Spinning_Piston.BP_Spinning_Piston_C|SetIsturning _asbp_spinning_piston true))
    (:then_3
      (bind _asbp_rotating_blade_2 (Utilities|Casting|CastToBP_Rotating_Blade2 OtherActor))
      (Variables|/Game/DemoGame/BPMAP2/Traps/BP_Rotating_Blade2.BP_Rotating_Blade2_C|SetTurning _asbp_rotating_blade_2 true)
      (Default|Start3 _asbp_rotating_blade_2))
    (:then_4
      (bind _asbp_rotating_blade (Utilities|Casting|CastToBP_Rotating_Blade OtherActor))
      (Variables|/Game/DemoGame/BPMAP2/Traps/BP_Rotating_Blade.BP_Rotating_Blade_C|SetTurning _asbp_rotating_blade true)
      (Default|Start4 _asbp_rotating_blade))
    (:then_5
      (bind _asbp_enemy_1 (Utilities|Casting|CastToBP_Enemy_1 OtherActor))
      (Default|Stop _asbp_enemy_1))))

(event EventBeginPlay
  (|CallParentFunction))

(event Collision|EventActorBeginOverlap
  (params (OtherActor :type Actor%20Object%20Reference))
  (|CallParentFunction OtherActor) ; This node is disabled and will not be called.\nDrag off pins to build functionality.
)

(event EventTick
  (params (DeltaSeconds :type Float%20%28single-precision%29))
  (|CallParentFunction DeltaSeconds) ; This node is disabled and will not be called.\nDrag off pins to build functionality.
)

(fn ConstructionScript
  (|CallParentFunction))