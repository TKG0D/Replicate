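; BP_Ammo is a one-time ammo pickup that responds to an Interaction event.
; If the player character's Ammo is below 10, a DoOnce lets it add 10 to that value and call Reload on the character.
; It then destroys only its StaticMesh component, leaving the actor itself in place.
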(event EventTick
  (params (DeltaSeconds :type Float%20%28single-precision%29)))

(event Collision|EventActorBeginOverlap
  (params (OtherActor :type Actor%20Object%20Reference)))

(event EventInteraction
  (bind _asbp_third_person_character (Utilities|Casting|CastToBP_ThirdPersonCharacter (Game|GetPlayerCharacter 0)))
  (if (< (Variables|/Game/ThirdPerson/Blueprints/BP_ThirdPersonCharacter.BP_ThirdPersonCharacter_C|GetAmmo _asbp_third_person_character) 10)
    (Utilities|FlowControl|DoOnce false
      (:Completed
        (bind _asbp_third_person_character_2 (Utilities|Casting|CastToBP_ThirdPersonCharacter (Game|GetPlayerCharacter 0)))
        (Variables|/Game/ThirdPerson/Blueprints/BP_ThirdPersonCharacter.BP_ThirdPersonCharacter_C|SetAmmo _asbp_third_person_character_2 (+ (Variables|/Game/ThirdPerson/Blueprints/BP_ThirdPersonCharacter.BP_ThirdPersonCharacter_C|GetAmmo _asbp_third_person_character_2) 10))
        (Default|Reload _asbp_third_person_character_2)
        (Components|DestroyComponent (Variables|Default|GetStaticMesh))))))

(fn ConstructionScript)