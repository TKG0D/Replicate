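; Trigger volume that springs a laser trap the first time BP_ThirdPersonCharacter overlaps its box.
; A timeline lowers the referenced Door's mesh while four referenced trap cubes become visible and slide along local Y on separate timelines.
; Each trap timeline restarts two seconds after finishing, so the sweeps repeat endlessly; the 0–100 loop around PlayFromStart only re-issues the same restart instantly.
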(event OnComponentBeginOverlap(Box)
  (params (OverlappedComponent :type Primitive%20Component%20Object%20Reference) (OtherActor :type Actor%20Object%20Reference) (OtherComp :type Primitive%20Component%20Object%20Reference) (OtherBodyIndex :type Integer) (bFromSweep :type Boolean) (SweepResult :type Hit%20Result%20Structure%20%28by%20ref%29))
  (Utilities|Casting|CastToBP_ThirdPersonCharacter OtherActor)
  (Utilities|FlowControl|Sequence
    (:then_0
      (Utilities|FlowControl|DoOnce false
        (:Completed
          (bind _newtrack_0 (Timeline|Timeline Play)
            (:Update
              (Transformation|SetRelativeLocation (Variables|/Game/DemoGame/BPMAP2/Traps/BP_Trap_Door.BP_Trap_Door_C|GetStaticMesh (Variables|Default|GetDoor)) (Math|Vector|Lerp(Vector) "0, 0, 0" "0.000000,0.000000,-220.000000" _newtrack_0) false false))))))
    (:then_1
      (Utilities|FlowControl|DoOnce false
        (:Completed
          (Utilities|FlowControl|Sequence
            (:then_0
              (Rendering|SetVisibility (Variables|/Game/DemoGame/BPMAP2/Traps/BP_laser_Trap.BP_laser_Trap_C|GetCube (Variables|Default|GetTrap)) true false)
              (Utilities|FlowControl|Sequence
                (:then_0
                  (bind _newtrack_0_2 (Timeline|Timeline_0 Play)
                    (:Update
                      (Transformation|SetRelativeLocation (Variables|/Game/DemoGame/BPMAP2/Traps/BP_laser_Trap.BP_laser_Trap_C|GetCube (Variables|Default|GetTrap)) (Math|Vector|Lerp(Vector) "0, 0, 0" "0.000000,4615.000000,0.000000" _newtrack_0_2) false false))
                    (:Finished
                      (Utilities|FlowControl|Delay 2.0)
                      (for _index (range 0 100)
                        (Timeline|Timeline_0 PlayFromStart)))))
                (:then_1
                  (bind _newtrack_0_3 (Timeline|Timeline_1 Play)
                    (:Update
                      (Transformation|SetRelativeLocation (Variables|/Game/DemoGame/BPMAP2/Traps/BP_laser_Trap.BP_laser_Trap_C|GetCube (Variables|Default|GetTrap_0)) (Math|Vector|Lerp(Vector) "0, 0, 0" "0.000000,4615.000000,0.000000" _newtrack_0_3) false false))
                    (:Finished
                      (Utilities|FlowControl|Delay 2.0)
                      (for _index_2 (range 0 100)
                        (Timeline|Timeline_1 PlayFromStart)))))
                (:then_2
                  (bind _newtrack_0_4 (Timeline|Timeline_2 Play)
                    (:Update
                      (Transformation|SetRelativeLocation (Variables|/Game/DemoGame/BPMAP2/Traps/BP_laser_Trap.BP_laser_Trap_C|GetCube (Variables|Default|GetTrap_1)) (Math|Vector|Lerp(Vector) "0, 0, 0" "0.000000,4615.000000,0.000000" _newtrack_0_4) false false))
                    (:Finished
                      (Utilities|FlowControl|Delay 2.0)
                      (for _index_3 (range 0 100)
                        (Timeline|Timeline_2 PlayFromStart)))))
                (:then_3
                  (bind _newtrack_0_5 (Timeline|Timeline_3 Play)
                    (:Update
                      (Transformation|SetRelativeLocation (Variables|/Game/DemoGame/BPMAP2/Traps/BP_laser_Trap.BP_laser_Trap_C|GetCube (Variables|Default|GetTrap_2)) (Math|Vector|Lerp(Vector) "0, 0, 0" "0.000000,4615.000000,0.000000" _newtrack_0_5) false false))
                    (:Finished
                      (Utilities|FlowControl|Delay 2.0)
                      (for _index_4 (range 0 100)
                        (Timeline|Timeline_3 PlayFromStart)))))))
            (:then_1
              (Rendering|SetVisibility (Variables|/Game/DemoGame/BPMAP2/Traps/BP_laser_Trap.BP_laser_Trap_C|GetCube (Variables|Default|GetTrap_0)) true false))
            (:then_2
              (Rendering|SetVisibility (Variables|/Game/DemoGame/BPMAP2/Traps/BP_laser_Trap.BP_laser_Trap_C|GetCube (Variables|Default|GetTrap_1)) true false))
            (:then_3
              (Rendering|SetVisibility (Variables|/Game/DemoGame/BPMAP2/Traps/BP_laser_Trap.BP_laser_Trap_C|GetCube (Variables|Default|GetTrap_2)) true false))))))))

(event EventBeginPlay)

(event Collision|EventActorBeginOverlap
  (params (OtherActor :type Actor%20Object%20Reference)))

(event EventTick
  (params (DeltaSeconds :type Float%20%28single-precision%29)))

(fn ConstructionScript)