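; BP_Switch is a trigger actor that opens a linked door once the key condition is met.
; A Gotkey2 event sets the Haskey flag, which gates the box overlap check for BP_ThirdPersonCharacter.
; A valid overlap prints a debug message and plays a timeline that lerps the door's cube upward in relative space.
; Nothing in the graph reverses the movement or clears the flag.
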(event OnComponentBeginOverlap(Box)
  (params (OverlappedComponent :type Primitive%20Component%20Object%20Reference) (OtherActor :type Actor%20Object%20Reference) (OtherComp :type Primitive%20Component%20Object%20Reference) (OtherBodyIndex :type Integer) (bFromSweep :type Boolean) (SweepResult :type Hit%20Result%20Structure%20%28by%20ref%29))
  (Utilities|Casting|CastToBP_ThirdPersonCharacter OtherActor)
  (if (Variables|Default|GetHaskey)
    (Development|PrintString "Hello")
    (bind _newtrack_0 (Timeline|Timeline Play)
      (:Update
        (Transformation|SetRelativeLocation (Variables|/Game/DemoGame/BPMAP2/Doors/BP_DoorLocked.BP_DoorLocked_C|GetCube (Variables|Default|GetDoor)) (Math|Vector|Lerp(Vector) "0, 0, 0" "0.000000,0.000000,200.000000" _newtrack_0) false false)))))

(event Custom|Gotkey2
  (Variables|Default|SetHaskey true))

(event EventBeginPlay)

(event Collision|EventActorBeginOverlap
  (params (OtherActor :type Actor%20Object%20Reference)))

(event EventTick
  (params (DeltaSeconds :type Float%20%28single-precision%29)))

(fn ConstructionScript)