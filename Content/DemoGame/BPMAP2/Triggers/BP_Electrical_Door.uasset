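; Electrical door trigger that opens a linked ElectricDoor when the third-person character enters its box while four referenced actors are all switched on.
; The overlap checks each actor's On flag, clears LaserOn, then passes through a DoOnce into a timeline.
; The timeline lerps the door's cube upward in relative space, with no closing logic.
; An unconnected sequence that would apply Neon materials to the cube never runs.
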(event OnComponentBeginOverlap(Box)
  (params (OverlappedComponent :type Primitive%20Component%20Object%20Reference) (OtherActor :type Actor%20Object%20Reference) (OtherComp :type Primitive%20Component%20Object%20Reference) (OtherBodyIndex :type Integer) (bFromSweep :type Boolean) (SweepResult :type Hit%20Result%20Structure%20%28by%20ref%29))
  (Utilities|Casting|CastToBP_ThirdPersonCharacter OtherActor)
  (if (Math|Boolean|ANDBoolean (Variables|/Game/DemoGame/BPMAP2/Triggers/DoorSwitchElectrical.DoorSwitchElectrical_C|GetOn (Variables|Default|GetDoor)) (Variables|/Game/DemoGame/BPMAP2/Triggers/DoorSwitchElectrical1.DoorSwitchElectrical1_C|GetOn1 (Variables|Default|GetDoor_0)) (Variables|/Game/DemoGame/BPMAP2/Triggers/DoorSwitchElectrical2.DoorSwitchElectrical2_C|GetOn2 (Variables|Default|GetDoor_1)) (Variables|/Game/DemoGame/BPMAP2/Triggers/DoorSwitchElectrical3.DoorSwitchElectrical3_C|GetOn3 (Variables|Default|GetDoor_2)))
    (Variables|Default|SetLaserOn false)
    (if (not (Variables|Default|GetLaserOn))
      (Utilities|FlowControl|DoOnce false
        (:Completed
          (bind _newtrack_0 (Timeline|Open%20Door Play)
            (:Update
              (Transformation|SetRelativeLocation (Variables|/Game/DemoGame/BPMAP2/Doors/BP_Electric_Door.BP_Electric_Door_C|GetCube (Variables|Default|GetElectricDoor)) (Math|Vector|Lerp(Vector) "0, 0, 0" "0.000000,0.000000,225.000000" _newtrack_0) false false))))))))

(fn ConstructionScript)