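; Wind tunnel trigger that pushes the player while they are inside volume A.
; Entering raises the player's walk speed and starts a looping timer; leaving lowers the speed and clears it.
; While RotatingBlade is not Turning, each tick of the timer sphere-traces along fifteen arrow components, with debug drawing on.
; Every trace hitting the player adds a velocity-change impulse along the first arrow's forward vector, whichever arrow hit.
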(event OnComponentBeginOverlap(a)
  (params (OverlappedComponent :type Primitive%20Component%20Object%20Reference) (OtherActor :type Actor%20Object%20Reference) (OtherComp :type Primitive%20Component%20Object%20Reference) (OtherBodyIndex :type Integer) (bFromSweep :type Boolean) (SweepResult :type Hit%20Result%20Structure%20%28by%20ref%29))
  (if (== OtherActor (Game|GetPlayerCharacter 0))
    (Variables|/Script/Engine.CharacterMovementComponent|SetMaxWalkSpeed (Actor|GetComponentbyClass OtherActor "/Script/Engine.CharacterMovementComponent") 2e+03)
    (bind _returnvalue (Utilities|Time|SetTimerbyEvent (delegate Custom|CustomEvent) 0.2 true))
    (Variables|Default|SetNewVar _returnvalue)))

(event OnComponentEndOverlap(a)
  (params (OverlappedComponent :type Primitive%20Component%20Object%20Reference) (OtherActor :type Actor%20Object%20Reference) (OtherComp :type Primitive%20Component%20Object%20Reference) (OtherBodyIndex :type Integer))
  (if (== OtherActor (Game|GetPlayerCharacter 0))
    (Variables|/Script/Engine.CharacterMovementComponent|SetMaxWalkSpeed (Actor|GetComponentbyClass OtherActor "/Script/Engine.CharacterMovementComponent") 5e+02)
    (Utilities|Time|ClearandInvalidateTimerbyHandle (Variables|Default|GetNewVar))))

(event Custom|CustomEvent
  (if (not (Variables|/Game/DemoGame/BPMAP2/Traps/BP_Rotating_Blade2.BP_Rotating_Blade2_C|GetTurning (Variables|Default|GetRotating%20Blade)))
    (for (_ _array_index) (Utilities|Array|MakeArray (Variables|Default|GetArrow) (Variables|Default|GetArrow1) (Variables|Default|GetArrow2) (Variables|Default|GetArrow3) (Variables|Default|GetArrow4) (Variables|Default|GetArrow5) (Variables|Default|GetArrow6) (Variables|Default|GetArrow7) (Variables|Default|GetArrow8) (Variables|Default|GetArrow9) (Variables|Default|GetArrow10) (Variables|Default|GetArrow11) (Variables|Default|GetArrow12) (Variables|Default|GetArrow13) (Variables|Default|GetArrow14))
      (bind (_outhit _returnvalue) (Collision|SphereTraceForObjects (Transformation|GetWorldLocation (Utilities|Select :Index _array_index :Option%200 (Variables|Default|GetArrow) :Option%201 (Variables|Default|GetArrow1) :Option%202 (Variables|Default|GetArrow2) :Option%203 (Variables|Default|GetArrow3) :Option%204 (Variables|Default|GetArrow4) :Option%205 (Variables|Default|GetArrow5) :Option%206 (Variables|Default|GetArrow6) :Option%207 (Variables|Default|GetArrow7) :Option%208 (Variables|Default|GetArrow8) :Option%209 (Variables|Default|GetArrow9) :Option%2010 (Variables|Default|GetArrow10) :Option%2011 (Variables|Default|GetArrow11) :Option%2012 (Variables|Default|GetArrow12) :Option%2013 (Variables|Default|GetArrow13) :Option%2014 (Variables|Default|GetArrow14) :Option%2015 0)) (+ (Transformation|GetWorldLocation (Utilities|Select :Index _array_index :Option%200 (Variables|Default|GetArrow) :Option%201 (Variables|Default|GetArrow1) :Option%202 (Variables|Default|GetArrow2) :Option%203 (Variables|Default|GetArrow3) :Option%204 (Variables|Default|GetArrow4) :Option%205 (Variables|Default|GetArrow5) :Option%206 (Variables|Default|GetArrow6) :Option%207 (Variables|Default|GetArrow7) :Option%208 (Variables|Default|GetArrow8) :Option%209 (Variables|Default|GetArrow9) :Option%2010 (Variables|Default|GetArrow10) :Option%2011 (Variables|Default|GetArrow11) :Option%2012 (Variables|Default|GetArrow12) :Option%2013 (Variables|Default|GetArrow13) :Option%2014 (Variables|Default|GetArrow14) :Option%2015 0)) (* (Math|Vector|GetForwardVector (Utilities|Select :Index _array_index :Option%200 (Variables|Default|GetArrow) :Option%201 (Variables|Default|GetArrow1) :Option%202 (Variables|Default|GetArrow2) :Option%203 (Variables|Default|GetArrow3) :Option%204 (Variables|Default|GetArrow4) :Option%205 (Variables|Default|GetArrow5) :Option%206 (Variables|Default|GetArrow6) :Option%207 (Variables|Default|GetArrow7) :Option%208 (Variables|Default|GetArrow8) :Option%209 (Variables|Default|GetArrow9) :Option%2010 (Variables|Default|GetArrow10) :Option%2011 (Variables|Default|GetArrow11) :Option%2012 (Variables|Default|GetArrow12) :Option%2013 (Variables|Default|GetArrow13) :Option%2014 (Variables|Default|GetArrow14) :Option%2015 0)) (Variables|Default|GetLineExtent))) 75.0 (Utilities|Array|MakeArray "ObjectTypeQuery1" "ObjectTypeQuery2" "ObjectTypeQuery3" "ObjectTypeQuery4") false 0 "ForDuration"))
      (if (and (== (.HitActor (Collision|BreakHitResult _outhit)) (Game|GetPlayerCharacter 0)) _returnvalue)
        (Physics|AddImpulse (Actor|GetComponentbyClass (.HitActor (Collision|BreakHitResult _outhit)) "/Script/Engine.CharacterMovementComponent") (* (Math|Vector|GetForwardVector (Variables|Default|GetArrow)) 1e+03) true)))))

(fn ConstructionScript)