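; BP_Security_Button is a trigger that lowers a door when the player character enters its box and the referenced Button's Ultra flag is set.
; If Ultra is set, a one-time Timeline lerps the referenced Door's Cube downward in relative space.
; Otherwise, it shows a WB_Electrical_Grid widget on overlap and removes it when the character leaves.
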(event OnComponentBeginOverlap(Box)
  (params (OverlappedComponent :type Primitive%20Component%20Object%20Reference) (OtherActor :type Actor%20Object%20Reference) (OtherComp :type Primitive%20Component%20Object%20Reference) (OtherBodyIndex :type Integer) (bFromSweep :type Boolean) (SweepResult :type Hit%20Result%20Structure%20%28by%20ref%29))
  (Utilities|Casting|CastToBP_ThirdPersonCharacter OtherActor)
  (if (Variables|/Game/DemoGame/BPMAP2/Trigger2/BP_SecuritySwitch.BP_SecuritySwitch_C|GetUltra (Variables|Default|GetButton))
    (Utilities|FlowControl|DoOnce false
      (:Completed
        (bind _newtrack_0 (Timeline|Timeline Play)
          (:Update
            (Transformation|SetRelativeLocation (Variables|/Game/DemoGame/BPMAP2/Doors/BP_Securitiy_Door.BP_Securitiy_Door_C|GetCube (Variables|Default|GetDoor)) (Math|Vector|Lerp(Vector) "0, 0, 0" "0.000000,0.000000,-250.000000" _newtrack_0) false false)))))
    (else
      (bind _returnvalue (UserInterface|CreateWidget "/Game/DemoGame/Widgets/WB_Electrical_Grid.WB_Electrical_Grid_C"))
      (UserInterface|Viewport|AddtoViewport _returnvalue 0))))

(event OnComponentEndOverlap(Box)
  (params (OverlappedComponent :type Primitive%20Component%20Object%20Reference) (OtherActor :type Actor%20Object%20Reference) (OtherComp :type Primitive%20Component%20Object%20Reference) (OtherBodyIndex :type Integer))
  (Utilities|Casting|CastToBP_ThirdPersonCharacter OtherActor)
  (if (not (Variables|/Game/DemoGame/BPMAP2/Trigger2/BP_SecuritySwitch.BP_SecuritySwitch_C|GetUltra (Variables|Default|GetButton)))
    (Widget|RemovefromParent (stale OnComponentBeginOverlap(Box) _returnvalue))))

(event EventBeginPlay)

(fn ConstructionScript)