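; Middle-map console that, on its first interaction while usable, activates the area's systems in a one-time sequence.
; Timelines drive lerped relative moves that slide two middle laser meshes up and another referenced mesh and a door down.
; After a delay, both middle lasers start their rotating movement.
; The same sequence swaps neon materials on other lasers and the entrance, turns a light green and plays a systems-active sound.
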(event EventBeginPlay)

(event EventInteraction
  (if (Variables|/Game/DemoGame/BPMAP2/Triggers/BP_Elevator_Trigger.BP_Elevator_Trigger_C|GetIsConsoleUsable (Variables|Default|Getconsole))
    (Utilities|FlowControl|DoOnce false
      (:Completed
        (Utilities|FlowControl|Sequence
          (:then_0
            (bind _newtrack_0 (Timeline|Timeline Play)
              (:Update
                (Transformation|SetRelativeLocation (Variables|/Game/DemoGame/BPMAP2/Traps/BP_Laser_Mid.BP_Laser_Mid_C|GetCube (Variables|Default|GetLaserMid)) (Math|Vector|Lerp(Vector) "0, 0, 0" "0.000000,0.000000,1680.000000" _newtrack_0) false false)
                (Utilities|FlowControl|Delay 3.0)
                (Components|Activation|SetActive (Variables|/Game/DemoGame/BPMAP2/Traps/BP_Laser_Mid.BP_Laser_Mid_C|GetRotatingMovement (Variables|Default|GetLaserMid)) true false))))
          (:then_1
            (bind _newtrack_0_2 (Timeline|Timeline_0 Play)
              (:Update
                (Transformation|SetRelativeLocation (Variables|/Game/DemoGame/BPMAP2/Traps/BP_Laser_Mid.BP_Laser_Mid_C|GetCube (Variables|Default|GetLaserMid_0)) (Math|Vector|Lerp(Vector) "0, 0, 0" "0.000000,0.000000,1680.000000" _newtrack_0_2) false false)
                (Utilities|FlowControl|Delay 3.0)
                (Components|Activation|SetActive (Variables|/Game/DemoGame/BPMAP2/Traps/BP_Laser_Mid.BP_Laser_Mid_C|GetRotatingMovement (Variables|Default|GetLaserMid_0)) true false))))
          (:then_2
            (bind _newtrack_0_3 (Timeline|Timeline_1 Play)
              (:Update
                (Transformation|SetRelativeLocation (Variables|/Game/DemoGame/BPMAP2/BP_Entrance_Door.BP_Entrance_Door_C|GetCube (Variables|Default|GetNewVar)) (Math|Vector|Lerp(Vector) "0, 0, 0" "0.000000,0.000000,-1750.000000" _newtrack_0_3) false false))))
          (:then_3
            (Rendering|Material|SetMaterial (Variables|/Game/DemoGame/BPMAP2/Traps/BP_Laser_Mid.BP_Laser_Mid_C|GetCube2 (Variables|Default|GetLaser)) 0 "/Game/DemoGame/Materials/Neon3.Neon3"))
          (:then_4
            (Rendering|Material|SetMaterial (Variables|/Game/DemoGame/BPMAP2/Traps/BP_Laser_Mid.BP_Laser_Mid_C|GetCube3 (Variables|Default|GetLaser)) 0 "/Game/DemoGame/Materials/Neon3.Neon3"))
          (:then_5
            (Rendering|Material|SetMaterial (Variables|/Game/DemoGame/BPMAP2/Traps/BP_Laser_Mid.BP_Laser_Mid_C|GetCube2 (Variables|Default|GetLaser_0)) 0 "/Game/DemoGame/Materials/Neon3.Neon3"))
          (:then_6
            (Rendering|Material|SetMaterial (Variables|/Game/DemoGame/BPMAP2/Traps/BP_Laser_Mid.BP_Laser_Mid_C|GetCube3 (Variables|Default|GetLaser_0)) 0 "/Game/DemoGame/Materials/Neon3.Neon3"))
          (:then_7
            (Rendering|Material|SetMaterial (Variables|/Game/DemoGame/Decoration/AnswerPuzzle2.AnswerPuzzle2_C|GetCube (Variables|Default|GetEntrance)) 0 "/Game/DemoGame/Materials/Neon2.Neon2"))
          (:then_8
            (Rendering|Material|SetMaterial (Variables|/Game/DemoGame/Decoration/AnswerPuzzle2.AnswerPuzzle2_C|GetCube (Variables|Default|GetEntrance)) 1 "/Game/DemoGame/Materials/Neon2.Neon2"))
          (:then_9
            (Rendering|Material|SetMaterial (Variables|/Game/DemoGame/Decoration/AnswerPuzzle2.AnswerPuzzle2_C|GetCube1 (Variables|Default|GetEntrance)) 0 "/Game/DemoGame/Materials/Neon2.Neon2"))
          (:then_10
            (Rendering|Material|SetMaterial (Variables|/Game/DemoGame/Decoration/AnswerPuzzle2.AnswerPuzzle2_C|GetCube1 (Variables|Default|GetEntrance)) 1 "/Game/DemoGame/Materials/Neon2.Neon2"))
          (:then_11
            (Rendering|Material|SetMaterial (Variables|/Game/DemoGame/Decoration/AnswerPuzzle2.AnswerPuzzle2_C|GetStaticMesh (Variables|Default|GetEntrance)) 0 "/Game/DemoGame/Materials/Neon2.Neon2"))
          (:then_12
            (Rendering|Material|SetMaterial (Variables|/Game/DemoGame/Decoration/AnswerPuzzle2.AnswerPuzzle2_C|GetStaticMesh (Variables|Default|GetEntrance)) 1 "/Game/DemoGame/Materials/Neon2.Neon2"))
          (:then_13
            (Rendering|Components|Light|SetLightColor (Variables|/Script/Engine.Light|GetLightComponent (Variables|Default|GetLight)) "(R=0.037358,G=1.000000,B=0.000000,A=1.000000)" true))
          (:then_14
            (bind _newtrack_0_4 (Timeline|Timeline_2 Play)
              (:Update
                (Transformation|SetRelativeLocation (Variables|/Game/DemoGame/BPMAP2/Doors/BP_Door_Sector2.BP_Door_Sector2_C|GetCube (Variables|Default|GetDoor)) (Math|Vector|Lerp(Vector) "0, 0, 0" "0.000000,0.000000,-250.000000" _newtrack_0_4) false false))))
          (:then_15
            (Audio|PlaySound2D "/Game/DemoGame/BPMAP2/Sounds/All_Systems_Active_Sound_Effect.All_Systems_Active_Sound_Effect" 1.0 1.0 0.0 0 0)))))))

(fn ConstructionScript)