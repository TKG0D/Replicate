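; BP_Rotating_Blade is a trap that spins via RotatingMovement from BeginPlay and can be temporarily frozen by the Start4 event.
; When Turning is true, Start4 swaps five meshes to a pulsing hex material, stops rotation and plays a stasis sound.
; After a two-second delay it resumes rotation, restores the metal material and clears Turning, which this graph never sets true.
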(event Custom|Start4
  (if (Variables|Default|GetTurning)
    (Utilities|FlowControl|Sequence
      (:then_0
        (Rendering|Material|SetMaterial (Variables|Default|GetCube) 0 "/Game/StarterContent/Materials/M_Tech_Hex_Tile_Pulse.M_Tech_Hex_Tile_Pulse")
        (Components|Activation|Deactivate (Variables|Default|GetRotatingMovement))
        (Audio|PlaySound2D "/Game/DemoGame/BPMAP2/Sounds/BotW__Stasis_to_Temple_of_Time_-_Boulder_Strat-_AudioTrimmer_com_.BotW__Stasis_to_Temple_of_Time_-_Boulder_Strat-_AudioTrimmer_com_" 1.0 1.0 0.0 0 0)
        (Utilities|FlowControl|Delay 2.0)
        (Components|Activation|Activate (Variables|Default|GetRotatingMovement) false)
        (Variables|Default|SetTurning false)
        (Development|PrintString "Gear Resume")
        (Utilities|FlowControl|Sequence
          (:then_0
            (Rendering|Material|SetMaterial (Variables|Default|GetCube) 0 "/Game/Sbsar_Material/Material/Black_Space_Metal.Black_Space_Metal"))
          (:then_1
            (Rendering|Material|SetMaterial (Variables|Default|GetStaticMesh1) 0 "/Game/Sbsar_Material/Material/Black_Space_Metal.Black_Space_Metal"))
          (:then_2
            (Rendering|Material|SetMaterial (Variables|Default|GetStaticMesh2) 0 "/Game/Sbsar_Material/Material/Black_Space_Metal.Black_Space_Metal"))
          (:then_3
            (Rendering|Material|SetMaterial (Variables|Default|GetCube1) 0 "/Game/Sbsar_Material/Material/Black_Space_Metal.Black_Space_Metal"))
          (:then_4
            (Rendering|Material|SetMaterial (Variables|Default|GetStaticMesh) 0 "/Game/Sbsar_Material/Material/Black_Space_Metal.Black_Space_Metal"))))
      (:then_1
        (Rendering|Material|SetMaterial (Variables|Default|GetCube1) 0 "/Game/StarterContent/Materials/M_Tech_Hex_Tile_Pulse.M_Tech_Hex_Tile_Pulse"))
      (:then_2
        (Rendering|Material|SetMaterial (Variables|Default|GetStaticMesh) 0 "/Game/StarterContent/Materials/M_Tech_Hex_Tile_Pulse.M_Tech_Hex_Tile_Pulse"))
      (:then_3
        (Rendering|Material|SetMaterial (Variables|Default|GetStaticMesh1) 0 "/Game/StarterContent/Materials/M_Tech_Hex_Tile_Pulse.M_Tech_Hex_Tile_Pulse"))
      (:then_4
        (Rendering|Material|SetMaterial (Variables|Default|GetStaticMesh2) 0 "/Game/StarterContent/Materials/M_Tech_Hex_Tile_Pulse.M_Tech_Hex_Tile_Pulse")))))

(event EventBeginPlay
  (Components|Activation|Activate (Variables|Default|GetRotatingMovement) false))

(fn ConstructionScript)