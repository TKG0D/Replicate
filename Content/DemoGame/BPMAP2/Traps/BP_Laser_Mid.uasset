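; Rotating laser trap for Map2 that destroys the third-person character on contact and reloads the level.
; Several box overlaps act as kill zones: two show a Tenti widget and reload immediately, others reload after a delay, while Box2 and Box3 are empty.
; Start2, gated by Isturning, briefly halts the RotatingMovement with a pulsing cube material, then resumes, restores the material and clears the flag.
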(event OnComponentBeginOverlap(Box6)
  (params (OverlappedComponent :type Primitive%20Component%20Object%20Reference) (OtherActor :type Actor%20Object%20Reference) (OtherComp :type Primitive%20Component%20Object%20Reference) (OtherBodyIndex :type Integer) (bFromSweep :type Boolean) (SweepResult :type Hit%20Result%20Structure%20%28by%20ref%29))
  (bind _asbp_third_person_character (Utilities|Casting|CastToBP_ThirdPersonCharacter OtherActor))
  (Actor|DestroyActor _asbp_third_person_character)
  (Utilities|FlowControl|Delay 2.0)
  (Game|OpenLevel(byName) "Map2"))

(event OnComponentBeginOverlap(Box7)
  (params (OverlappedComponent :type Primitive%20Component%20Object%20Reference) (OtherActor :type Actor%20Object%20Reference) (OtherComp :type Primitive%20Component%20Object%20Reference) (OtherBodyIndex :type Integer) (bFromSweep :type Boolean) (SweepResult :type Hit%20Result%20Structure%20%28by%20ref%29))
  (bind _asbp_third_person_character (Utilities|Casting|CastToBP_ThirdPersonCharacter OtherActor))
  (Actor|DestroyActor _asbp_third_person_character)
  (Utilities|FlowControl|Delay 2.0)
  (Game|OpenLevel(byName) "Map2"))

(event OnComponentBeginOverlap(Box8)
  (params (OverlappedComponent :type Primitive%20Component%20Object%20Reference) (OtherActor :type Actor%20Object%20Reference) (OtherComp :type Primitive%20Component%20Object%20Reference) (OtherBodyIndex :type Integer) (bFromSweep :type Boolean) (SweepResult :type Hit%20Result%20Structure%20%28by%20ref%29))
  (bind _asbp_third_person_character (Utilities|Casting|CastToBP_ThirdPersonCharacter OtherActor))
  (Actor|DestroyActor _asbp_third_person_character)
  (Utilities|FlowControl|Delay 2.0)
  (Game|OpenLevel(byName) "Map2"))

(event OnComponentBeginOverlap(Box)
  (params (OverlappedComponent :type Primitive%20Component%20Object%20Reference) (OtherActor :type Actor%20Object%20Reference) (OtherComp :type Primitive%20Component%20Object%20Reference) (OtherBodyIndex :type Integer) (bFromSweep :type Boolean) (SweepResult :type Hit%20Result%20Structure%20%28by%20ref%29))
  (bind _asbp_third_person_character (Utilities|Casting|CastToBP_ThirdPersonCharacter OtherActor))
  (Actor|DestroyActor _asbp_third_person_character)
  (bind _returnvalue (UserInterface|CreateWidget "/Game/DemoGame/BPMAP2/Widgets/Tenti.Tenti_C"))
  (UserInterface|Viewport|AddtoViewport _returnvalue 0)
  (Game|OpenLevel(byName) "Map2"))

(event OnComponentBeginOverlap(Box1)
  (params (OverlappedComponent :type Primitive%20Component%20Object%20Reference) (OtherActor :type Actor%20Object%20Reference) (OtherComp :type Primitive%20Component%20Object%20Reference) (OtherBodyIndex :type Integer) (bFromSweep :type Boolean) (SweepResult :type Hit%20Result%20Structure%20%28by%20ref%29))
  (bind _asbp_third_person_character (Utilities|Casting|CastToBP_ThirdPersonCharacter OtherActor))
  (Actor|DestroyActor _asbp_third_person_character)
  (bind _returnvalue (UserInterface|CreateWidget "/Game/DemoGame/BPMAP2/Widgets/Tenti.Tenti_C"))
  (UserInterface|Viewport|AddtoViewport _returnvalue 0)
  (Game|OpenLevel(byName) "Map2"))

(event OnComponentBeginOverlap(Box2)
  (params (OverlappedComponent :type Primitive%20Component%20Object%20Reference) (OtherActor :type Actor%20Object%20Reference) (OtherComp :type Primitive%20Component%20Object%20Reference) (OtherBodyIndex :type Integer) (bFromSweep :type Boolean) (SweepResult :type Hit%20Result%20Structure%20%28by%20ref%29)))

(event OnComponentBeginOverlap(Box3)
  (params (OverlappedComponent :type Primitive%20Component%20Object%20Reference) (OtherActor :type Actor%20Object%20Reference) (OtherComp :type Primitive%20Component%20Object%20Reference) (OtherBodyIndex :type Integer) (bFromSweep :type Boolean) (SweepResult :type Hit%20Result%20Structure%20%28by%20ref%29)))

(event OnComponentBeginOverlap(Box4)
  (params (OverlappedComponent :type Primitive%20Component%20Object%20Reference) (OtherActor :type Actor%20Object%20Reference) (OtherComp :type Primitive%20Component%20Object%20Reference) (OtherBodyIndex :type Integer) (bFromSweep :type Boolean) (SweepResult :type Hit%20Result%20Structure%20%28by%20ref%29))
  (bind _asbp_third_person_character (Utilities|Casting|CastToBP_ThirdPersonCharacter OtherActor))
  (Actor|DestroyActor _asbp_third_person_character)
  (Utilities|FlowControl|Delay 2.0)
  (Game|OpenLevel(byName) "Map2"))

(event OnComponentBeginOverlap(Box5)
  (params (OverlappedComponent :type Primitive%20Component%20Object%20Reference) (OtherActor :type Actor%20Object%20Reference) (OtherComp :type Primitive%20Component%20Object%20Reference) (OtherBodyIndex :type Integer) (bFromSweep :type Boolean) (SweepResult :type Hit%20Result%20Structure%20%28by%20ref%29))
  (bind _asbp_third_person_character (Utilities|Casting|CastToBP_ThirdPersonCharacter OtherActor))
  (Actor|DestroyActor _asbp_third_person_character)
  (Utilities|FlowControl|Delay 2.0)
  (Game|OpenLevel(byName) "Map2"))

(event Custom|Start2
  (if (Variables|Default|GetIsturning)
    (Rendering|Material|SetMaterial (Variables|Default|GetCube) 0 "/Game/StarterContent/Materials/M_Tech_Hex_Tile_Pulse.M_Tech_Hex_Tile_Pulse")
    (Components|Activation|Deactivate (Variables|Default|GetRotatingMovement))
    (Utilities|FlowControl|Delay 2.0)
    (Components|Activation|Activate (Variables|Default|GetRotatingMovement) false)
    (Variables|Default|SetIsturning false)
    (Development|PrintString "Gear Resume")
    (Rendering|Material|SetMaterial (Variables|Default|GetCube) 0 "/Game/SuperGrid/StarterPack/Materials/Palette/Grids/M_SuperGrid_Default.M_SuperGrid_Default")))

(event EventBeginPlay)

(event Collision|EventActorBeginOverlap
  (params (OtherActor :type Actor%20Object%20Reference)))

(fn ConstructionScript)