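; BP_Flying_Enemy is a flying homing enemy that destroys the third-person player on contact.
; KillPlayer, gated by an Enemy InArea flag, fires once to swap the cube material and aim ProjectileMovement homing at the player's mesh.
; Box overlap with the player explodes the enemy and opens Map2 after a delay.
; Overlap with a BP_Floor explodes it, removing cube and box and zeroing homing acceleration and velocity.
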(event OnComponentBeginOverlap(Box)
  (params (OverlappedComponent :type Primitive%20Component%20Object%20Reference) (OtherActor :type Actor%20Object%20Reference) (OtherComp :type Primitive%20Component%20Object%20Reference) (OtherBodyIndex :type Integer) (bFromSweep :type Boolean) (SweepResult :type Hit%20Result%20Structure%20%28by%20ref%29))
  (bind _projectilemovement (Variables|Default|GetProjectileMovement))
  (Utilities|FlowControl|Sequence
    (:then_0
      (bind _asbp_third_person_character (Utilities|Casting|CastToBP_ThirdPersonCharacter OtherActor))
      (Actor|DestroyActor _asbp_third_person_character)
      (Components|DestroyComponent (Variables|Default|GetCube))
      (Effects|SpawnEmitteratLocation "/Game/StarterContent/Particles/P_Explosion.P_Explosion" "0, 0, 0")
      (Audio|SpawnSound2D "/Game/StarterContent/Audio/Explosion01.Explosion01" 1.0 1.0 0.0 0)
      (Utilities|FlowControl|Delay 3.0)
      (Game|OpenLevel(byName) "Map2"))
    (:then_1
      (Utilities|Casting|CastToBP_Floor OtherActor)
      (Components|DestroyComponent (Variables|Default|GetCube))
      (Components|DestroyComponent (Variables|Default|GetBox))
      (Effects|SpawnEmitteratLocation "/Game/StarterContent/Particles/P_Explosion.P_Explosion" (.Location (Collision|BreakHitResult SweepResult)))
      (Audio|SpawnSound2D "/Game/StarterContent/Audio/Explosion01.Explosion01" 1.0 1.0 0.0 0)
      (Development|PrintString "Hello")
      (Variables|/Script/Engine.ProjectileMovementComponent|SetHomingAccelerationMagnitude _projectilemovement 0.0)
      (Variables|/Script/Engine.MovementComponent|SetVelocity _projectilemovement "0, 0, 0"))))

(event Custom|KillPlayer
  (bind _projectilemovement (Variables|Default|GetProjectileMovement))
  (bind _asbp_third_person_character (Utilities|Casting|CastToBP_ThirdPersonCharacter (Game|GetPlayerCharacter 0)))
  (if (Variables|/Game/DemoGame/BPMAP2/Trigger2/BP_Enemy_Fly.BP_Enemy_Fly_C|GetInArea (Variables|Default|GetEnemy))
    (Utilities|FlowControl|DoOnce false
      (:Completed
        (Rendering|Material|SetMaterial (Variables|Default|GetCube) 0 "/Game/StarterContent/Materials/M_Tech_Hex_Tile_Pulse.M_Tech_Hex_Tile_Pulse")
        (Variables|/Script/Engine.ProjectileMovementComponent|SetHomingTargetComponent _projectilemovement (Variables|/Script/Engine.Character|GetMesh _asbp_third_person_character))
        (Variables|/Script/Engine.ProjectileMovementComponent|SetHomingAccelerationMagnitude _projectilemovement 5e+03)
        (Variables|/Script/Engine.MovementComponent|SetVelocity _projectilemovement "0, 0, 0")))))

(event Collision|EventActorBeginOverlap
  (params (OtherActor :type Actor%20Object%20Reference)))

(event EventTick
  (params (DeltaSeconds :type Float%20%28single-precision%29)))

(fn ConstructionScript)