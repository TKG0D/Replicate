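; Base item actor that players can interact with to inspect, with mesh, scale, name and description set per item.
; The construction script applies the item mesh and scale to its static mesh component.
; On Interaction, if Inspect is enabled, it spawns a BP_Inspect_Item far away from the level.
; It passes that actor the mesh, text, interacting character and inspection rotation and scale.
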(event EventInteraction
  (params (Character :type BP%20Third%20Person%20Character%20Object%20Reference))
  (if (Variables|Default|GetInspect?)
    (bind _returnvalue (Game|SpawnActorfromClass "/Game/DemoGame/BPMAP2/Inspect/BP_Inspect_Item.BP_Inspect_Item_C" (Math|Transform|MakeTransform "100000000.000000,0.000000,0.000000") "Undefined" "MultiplyWithRoot" 0 0))
    (Default|SetInspectRotation _returnvalue (Variables|Default|GetItem%20Inspection%20Rotation))
    (Default|SetInspectScale _returnvalue (Variables|Default|GetItem%20Inspection%20Scale))
    (Class|BPIInteraction|Inspect(Message) _returnvalue Character (Variables|/Script/Engine.StaticMeshComponent|GetStaticMesh (Variables|Default|GetStaticMesh)) (Variables|Default|GetItem%20Name) (Variables|Default|GetItem%20Description))))

(fn ConstructionScript
  (bind _staticmesh (Variables|Default|GetStaticMesh))
  (Components|StaticMesh|SetStaticMesh _staticmesh (Variables|Default|GetItem%20Mesh))
  (Transformation|SetWorldTransform _staticmesh (Math|Transform|MakeTransform (Transformation|GetWorldLocation _staticmesh) (Transformation|GetWorldRotation _staticmesh) (Variables|Default|GetItem%20Scale)) false false))