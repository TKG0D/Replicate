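; BP_Key is a key pickup that unlocks progress on interaction by notifying three referenced objects, one of them a Door, that the key is obtained.
; Interaction sends those notifications on every call, then a DoOnce shows the BP_Acquired_Key widget and hides the key's meshes.
; The custom RemoveFromParent event waits briefly, then clears the widget and destroys the actor.
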(event Custom|RemoveFromParent
  (Utilities|FlowControl|Delay 1.0)
  (Widget|RemovefromParent (stale EventInteraction _returnvalue))
  (Actor|DestroyActor))

(event EventBeginPlay)

(event Collision|EventActorBeginOverlap
  (params (OtherActor :type Actor%20Object%20Reference)))

(event EventTick
  (params (DeltaSeconds :type Float%20%28single-precision%29)))

(event EventInteraction
  (Default|GotKey (Variables|Default|Getdoor))
  (Default|Gotkey2 (Variables|Default|GetNewVar))
  (Default|Gotkey3 (Variables|Default|GetNewVar_0))
  (Utilities|FlowControl|DoOnce false
    (:Completed
      (bind _returnvalue (UserInterface|CreateWidget "/Game/DemoGame/BPMAP2/Widgets/BP_Acquired_Key.BP_Acquired_Key_C"))
      (UserInterface|Viewport|AddtoViewport _returnvalue 0)
      (CallFunction|RemovefromParent)
      (Rendering|SetVisibility (Variables|Default|GetCube) false false)
      (Rendering|SetVisibility (Variables|Default|GetStaticMesh) false false)
      (Rendering|SetVisibility (Variables|Default|GetStaticMesh1) false false)
      (Rendering|SetVisibility (Variables|Default|GetStaticMesh2) false false)
      (Rendering|SetVisibility (Variables|Default|GetStaticMesh3) false false))))

(fn ConstructionScript)