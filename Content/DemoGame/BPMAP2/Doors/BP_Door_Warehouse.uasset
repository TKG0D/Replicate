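; BP_Door_Warehouse is a warehouse door that slides upward once electricity has unlocked it.
; The OpenDoorElectricity event sets HasKey, and a player character entering the Box trigger then opens the door a single time via DoOnce.
; A timeline lerps the Cube mesh's relative height while a pneumatic door sound plays in 2D.
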(event OnComponentBeginOverlap(Box)
  (params (OverlappedComponent :type Primitive%20Component%20Object%20Reference) (OtherActor :type Actor%20Object%20Reference) (OtherComp :type Primitive%20Component%20Object%20Reference) (OtherBodyIndex :type Integer) (bFromSweep :type Boolean) (SweepResult :type Hit%20Result%20Structure%20%28by%20ref%29))
  (Utilities|Casting|CastToBP_ThirdPersonCharacter OtherActor)
  (if (Variables|Default|GetHasKey)
    (Utilities|FlowControl|DoOnce false
      (:Completed
        (Utilities|FlowControl|Sequence
          (:then_0
            (bind _newtrack_0 (Timeline|Timeline Play)
              (:Update
                (Transformation|SetRelativeLocation (Variables|Default|GetCube) (Math|Vector|Lerp(Vector) "0, 0, 0" "0.000000,0.000000,1300.000000" _newtrack_0) false false))))
          (:then_1
            (Audio|PlaySound2D "/Game/DemoGame/BPMAP2/Sounds/Spaceship_compartment_door_with_pneumatics_Sound_Effect-_AudioTrimmer_com_.Spaceship_compartment_door_with_pneumatics_Sound_Effect-_AudioTrimmer_com_" 0.5 1.0 0.0 0 0)))))))

(event Custom|OpenDoorElectricity
  (Variables|Default|SetHasKey true))

(event EventBeginPlay)

(event Collision|EventActorBeginOverlap
  (params (OtherActor :type Actor%20Object%20Reference)))

(event EventTick
  (params (DeltaSeconds :type Float%20%28single-precision%29)))

(fn ConstructionScript)