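; BP_Door_WaitingArea1 is a waiting-area door that opens only when two referenced switches are both open.
; Its Openthedoor event checks both switch flags, then plays a power-up sound and triggers a colour event on each of three referenced generators.
; A timeline then lerps the door's Cube upward in relative space, with no sweep and no closing logic.
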(event Custom|Openthedoor
  (if (and (Variables|/Game/DemoGame/BPMAP2/Triggers/DoorSwitch5.DoorSwitch5_C|GetOpen2 (Variables|Default|Getswitch2)) (Variables|/Game/DemoGame/BPMAP2/Triggers/DoorSwitch3.DoorSwitch3_C|GetOpen (Variables|Default|Getswitch)))
    (Utilities|FlowControl|Sequence
      (:then_0
        (Audio|PlaySound2D "/Game/DemoGame/BPMAP2/Sounds/Electronic_Power_Up_Weapon_Power_Up_Gun_Power_Up_sound_Effect-_AudioTrimmer_com_.Electronic_Power_Up_Weapon_Power_Up_Gun_Power_Up_sound_Effect-_AudioTrimmer_com_" 0.4 1.0 0.0 0 0))
      (:then_1
        (Default|Colour1 (Variables|Default|GetGenerator)))
      (:then_2
        (Default|Colour2 (Variables|Default|GetGenerator_0)))
      (:then_3
        (Default|Colour3 (Variables|Default|GetGenerator_1)))
      (:then_4
        (bind _newtrack_0 (Timeline|Timeline Play)
          (:Update
            (Transformation|SetRelativeLocation (Variables|Default|GetCube) (Math|Vector|Lerp(Vector) "0, 0, 0" "0.000000,0.000000,1500.000000" _newtrack_0) false false)))))))

(event EventBeginPlay)

(event Collision|EventActorBeginOverlap
  (params (OtherActor :type Actor%20Object%20Reference)))

(event EventTick
  (params (DeltaSeconds :type Float%20%28single-precision%29)))

(fn ConstructionScript)