(event EventBeginPlay
  (|CallParentFunction)
  (Input|EnableInput (Game|GetPlayerController 0)))

(event EventInteraction
  (Variables|Default|SetKeyOpen true)
  (Utilities|FlowControl|Sequence
    (:then_0
      (Rendering|SetVisibility (Variables|Default|GetCube) false false))
    (:then_1
      (Rendering|SetVisibility (Variables|Default|GetCube1) false false))
    (:then_2
      (Rendering|SetVisibility (Variables|Default|GetCube2) false false))
    (:then_3
      (Rendering|SetVisibility (Variables|Default|GetCube3) false false))
    (:then_4
      (Rendering|SetVisibility (Variables|Default|GetCube4) false false))
    (:then_5
      (bind _returnvalue (UserInterface|CreateWidget "/Game/DemoGame/Widgets/WB_You_Picked_Up_Key.WB_You_Picked_Up_Key_C"))
      (UserInterface|Viewport|AddtoViewport _returnvalue 0)
      (Utilities|FlowControl|Delay 5.0)
      (Widget|RemovefromParent _returnvalue))))

(event EventTick
  (params (DeltaSeconds :type Float%20%28single-precision%29)))

(event Collision|EventActorBeginOverlap
  (params (OtherActor :type Actor%20Object%20Reference)))

(fn ConstructionScript)