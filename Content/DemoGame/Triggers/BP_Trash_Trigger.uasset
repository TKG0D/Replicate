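; BP_Trash_Trigger is a trigger actor that opens a trash door and moves a trash shoot piece when the third-person character enters its Box.
; On overlap, one timeline slides the TrashDoor cube along local X immediately, while a second slides the TrashShoot1 cube a shorter distance after a brief delay.
; Both timelines lerp relative location without sweep, and nothing reverses them when the character leaves.
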(event OnComponentBeginOverlap(Box)
  (params (OverlappedComponent :type Primitive%20Component%20Object%20Reference) (OtherActor :type Actor%20Object%20Reference) (OtherComp :type Primitive%20Component%20Object%20Reference) (OtherBodyIndex :type Integer) (bFromSweep :type Boolean) (SweepResult :type Hit%20Result%20Structure%20%28by%20ref%29))
  (Utilities|Casting|CastToBP_ThirdPersonCharacter OtherActor)
  (Utilities|FlowControl|Sequence
    (:then_0
      (Utilities|FlowControl|Delay 1.0)
      (bind _newtrack_0 (Timeline|Timeline Play)
        (:Update
          (Transformation|SetRelativeLocation (Variables|/Game/DemoGame/Gates/BP_Trash_Gate.BP_Trash_Gate_C|GetCube (Variables|Default|GetTrashShoot1)) (Math|Vector|Lerp(Vector) "0, 0, 0" "200.000000,0.000000,0.000000" _newtrack_0) false false))))
    (:then_1
      (bind _newtrack_0_2 (Timeline|Timeline_0 Play)
        (:Update
          (Transformation|SetRelativeLocation (Variables|/Game/DemoGame/Gates/BP_Trash_Gaste.BP_Trash_Gaste_C|GetCube (Variables|Default|GetTrashDoor)) (Math|Vector|Lerp(Vector) "0, 0, 0" "400.000000,0.000000,0.000000" _newtrack_0_2) false false))))))

(event EventBeginPlay)

(event Collision|EventActorBeginOverlap
  (params (OtherActor :type Actor%20Object%20Reference)))

(event EventTick
  (params (DeltaSeconds :type Float%20%28single-precision%29)))

(fn ConstructionScript)