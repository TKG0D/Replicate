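; BP_Mid_Laser2 is a trigger volume that slides a referenced fence's cube aside once a console has been activated.
; When the third-person character overlaps the box, it checks IsTriggered on the first BP_Console found in the level.
; If set, a DoOnce leads to a short delay, then a Timeline lerps Fence2's cube along negative Y in relative space.
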(event OnComponentBeginOverlap(Box)
  (params (OverlappedComponent :type Primitive%20Component%20Object%20Reference) (OtherActor :type Actor%20Object%20Reference) (OtherComp :type Primitive%20Component%20Object%20Reference) (OtherBodyIndex :type Integer) (bFromSweep :type Boolean) (SweepResult :type Hit%20Result%20Structure%20%28by%20ref%29))
  (Utilities|Casting|CastToBP_ThirdPersonCharacter OtherActor)
  (bind _outactors (Actor|GetAllActorsOfClass "/Game/DemoGame/Decoration/Imported_Assets/BP_Console.BP_Console_C"))
  (if (Variables|/Game/DemoGame/Decoration/Imported_Assets/BP_Console.BP_Console_C|GetIs%20Triggered (Utilities|Array|Get(acopy) _outactors))
    (Utilities|FlowControl|DoOnce false
      (:Completed
        (Utilities|FlowControl|Delay 2.0)
        (bind _newtrack_0 (Timeline|Timeline Play)
          (:Update
            (Transformation|SetRelativeLocation (Variables|/Game/DemoGame/Traps/BP_Fence_Mid_2.BP_Fence_Mid_2_C|GetCube (Variables|Default|GetFence2)) (Math|Vector|Lerp(Vector) "0, 0, 0" "0.000000,-2000.000000,0.000000" _newtrack_0) false false)))))))

(event EventBeginPlay)

(event Collision|EventActorBeginOverlap
  (params (OtherActor :type Actor%20Object%20Reference)))

(event EventTick
  (params (DeltaSeconds :type Float%20%28single-precision%29)))

(fn ConstructionScript)