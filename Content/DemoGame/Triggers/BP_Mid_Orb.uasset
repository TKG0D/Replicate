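; BP_Mid_Orb is a one-shot trigger that activates a laser trap when its capsule is overlapped.
; The first overlap passes a DoOnce before the player character cast, then shows the WB_Security_Activated widget for a timed delay.
; After the widget is removed, a Timeline slides the LaserTrap's cube along X.
; A Delay and DoOnce on the Timeline's update reverse it from the end once.
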(event OnComponentBeginOverlap(Capsule)
  (params (OverlappedComponent :type Primitive%20Component%20Object%20Reference) (OtherActor :type Actor%20Object%20Reference) (OtherComp :type Primitive%20Component%20Object%20Reference) (OtherBodyIndex :type Integer) (bFromSweep :type Boolean) (SweepResult :type Hit%20Result%20Structure%20%28by%20ref%29))
  (Utilities|FlowControl|DoOnce false
    (:Completed
      (Utilities|Casting|CastToBP_ThirdPersonCharacter OtherActor)
      (bind _returnvalue (UserInterface|CreateWidget "/Game/DemoGame/Widgets/WB_Security_Activated.WB_Security_Activated_C"))
      (UserInterface|Viewport|AddtoViewport _returnvalue 0)
      (Utilities|FlowControl|Delay 7.0)
      (Widget|RemovefromParent _returnvalue)
      (bind _newtrack_1 (Timeline|Timeline Play)
        (:Update
          (Transformation|SetRelativeLocation (Variables|/Game/DemoGame/Traps/BP_Fence_Trap.BP_Fence_Trap_C|GetCube (Variables|Default|GetLaserTrap)) (Math|Vector|Lerp(Vector) "0, 0, 0" "1290.000000,0.000000,0.000000" _newtrack_1) false false)
          (Utilities|FlowControl|Delay 7.0)
          (Utilities|FlowControl|DoOnce false
            (:Completed
              (Timeline|Timeline ReverseFromEnd))))))))

(event EventBeginPlay)

(event Collision|EventActorBeginOverlap
  (params (OtherActor :type Actor%20Object%20Reference)))

(event EventTick
  (params (DeltaSeconds :type Float%20%28single-precision%29)))

(fn ConstructionScript)