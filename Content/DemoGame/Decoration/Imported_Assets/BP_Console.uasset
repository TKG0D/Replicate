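; Interactable console Blueprint that triggers a one-time security activation, moving a gate and two laser traps.
; On first Interaction, it shows the security-activated widget and immediately starts timelines that lerp both laser trap cubes upward along Z.
; After a short delay, it removes the widget, sets IsTriggered and runs another timeline that raises FirstGate's root.
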(event EventBeginPlay)

(event Collision|EventActorBeginOverlap
  (params (OtherActor :type Actor%20Object%20Reference)))

(event EventTick
  (params (DeltaSeconds :type Float%20%28single-precision%29)))

(event EventInteraction
  (Utilities|FlowControl|DoOnce false
    (:Completed
      (Utilities|FlowControl|Sequence
        (:then_0
          (bind _returnvalue (UserInterface|CreateWidget "/Game/DemoGame/Widgets/WB_Security_Activated.WB_Security_Activated_C"))
          (UserInterface|Viewport|AddtoViewport _returnvalue 0)
          (Utilities|FlowControl|Delay 3.0)
          (Widget|RemovefromParent _returnvalue)
          (Variables|Default|SetIs%20Triggered true)
          (bind _newtrack_0 (Timeline|Timeline Play)
            (:Update
              (Transformation|SetRelativeLocation (Variables|/Script/Engine.Actor|GetRootComponent (Variables|Default|GetFirstGate)) (Math|Vector|Lerp(Vector) "0, 0, 0" "0.000000,0.000000,400.000000" _newtrack_0) false false))))
        (:then_1
          (bind _newtrack_0_2 (Timeline|LaserMid Play)
            (:Update
              (Transformation|SetRelativeLocation (Variables|/Game/DemoGame/Decoration/Laser_Trap_Mid.Laser_Trap_Mid_C|GetCube (Variables|Default|GetLaserTrap)) (Math|Vector|Lerp(Vector) "0, 0, 0" "0.000000,0.000000,300.000000" _newtrack_0_2) false false))))
        (:then_2
          (bind _newtrack_0_3 (Timeline|Timeline_0 Play)
            (:Update
              (Transformation|SetRelativeLocation (Variables|/Game/DemoGame/Decoration/Laser_Trap_Mid.Laser_Trap_Mid_C|GetCube (Variables|Default|GetLaserTrap2)) (Math|Vector|Lerp(Vector) "0, 0, 0" "0.000000,0.000000,300.000000" _newtrack_0_3) false false))))))))

(fn ConstructionScript)